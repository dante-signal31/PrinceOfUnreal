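; LevelCamera is an orthographic level camera Blueprint with an editor framing guide and a red screen tint effect.
; Its construction script sizes BoundingBox from the camera's ortho width and aspect ratio to visualize the view area, then caches the camera's post-process settings as defaults.
; TintRed swaps in the red flash post-process settings, and RemoveTint restores the cached defaults.
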(fn ConstructionScript
  (Utilities|FlowControl|Sequence
    (:then_0
      (CallFunction|SetVisualAid))
    (:then_1
      (CallFunction|SavePostProcessDefaultSettings))))

(fn SetVisualAid
  (bind _camera (Variables|Default|GetCamera))
  (bind _orthowidth (Variables|/Script/Engine.CameraComponent|GetOrthoWidth _camera))
  (Components|Box|SetBoxExtent (Variables|Default|GetBoundingBox) (Math|Vector|MakeVector (/ _orthowidth 2.0) (Variables|Default|GetVisualAidBoxDepth) (/ _orthowidth (* (Variables|/Script/Engine.CameraComponent|GetAspectRatio _camera) 2.0))) false)
  (return))

(fn TintRed
  (Variables|/Script/Engine.CameraComponent|SetPostProcessSettings (Variables|Default|GetCamera) (Variables|Default|GetFlashRedPostProcessSettings)))

(fn SavePostProcessDefaultSettings
  (Variables|Default|SetDefaultPostProcessSettings (Variables|/Script/Engine.CameraComponent|GetPostProcessSettings (Variables|Default|GetCamera)))
  (return))

(fn RemoveTint
  (Variables|/Script/Engine.CameraComponent|SetPostProcessSettings (Variables|Default|GetCamera) (Variables|Default|GetDefaultPostProcessSettings)))