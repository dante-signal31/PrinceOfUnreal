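; Base Blueprint for 2D traps that react to the PrinceCharacter, meant to be subclassed for each trap type.
; ProximityZone overlaps set CurrentState and call TrapActivated or TrapDeactivated; these and the KillingZone events are placeholders that children override.
; Construction sets initial state, bordered or borderless ground sprite, and flipbook looping.
; Helpers play paired front/back flipbooks with sound, toggle corpse and damage signal visuals, and reload the level.
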(event OnComponentBeginOverlap(ProximityZone)
  (params (OtherActor :type Actor%20Object%20Reference) (OtherComp :type Primitive%20Component%20Object%20Reference) (OtherBodyIndex :type Integer) (bFromSweep :type Boolean) (SweepResult :type Hit%20Result%20Structure%20%28by%20ref%29))
  ;[1 1 1] Entering trap range
  (CallFunction|InitTrapActivation OtherActor))

(event OnComponentEndOverlap(ProximityZone)
  (params (OtherActor :type Actor%20Object%20Reference) (OtherComp :type Primitive%20Component%20Object%20Reference) (OtherBodyIndex :type Integer))
  ;[1 1 1] Leaving trap range
  (CallFunction|InitTrapDeactivation OtherActor))

(event OnComponentBeginOverlap(KillingZone)
  (params (OtherActor :type Actor%20Object%20Reference) (OtherComp :type Primitive%20Component%20Object%20Reference) (OtherBodyIndex :type Integer) (bFromSweep :type Boolean) (SweepResult :type Hit%20Result%20Structure%20%28by%20ref%29))
  ;[1 1 1] Into the killing zone (OVERRIDE THIS)
  (Development|PrintString "Use of not overriden BeginOverlap KillingZone"))

(event OnComponentEndOverlap(KillingZone)
  (params (OtherActor :type Actor%20Object%20Reference) (OtherComp :type Primitive%20Component%20Object%20Reference) (OtherBodyIndex :type Integer))
  ;[1 1 1] Out the killing zone (OVERRIDE THIS)
  (Development|PrintString "Use of not overriden EndOverlap KillingZone"))

(event Custom|TrapActivated
  ;[1 1 1] Trap activation (OVERRIDE THIS)
  (Development|PrintString "Use of not overriden TrapActivated"))

(event Custom|TrapDeactivated
  ;[1 1 1] Trap deactivation (OVERRIDE THIS)
  (Development|PrintString "Use of not overriden TrapDeactivated"))

(fn ConstructionScript
  (Utilities|FlowControl|Sequence
    (:then_0
      (Variables|Default|SetCurrentState (Variables|Default|GetInitialState))
      (Variables|Default|SetActivationFlipbookLengthUp (Class|PaperFlipbookComponent|GetFlipbookLengthinFrames (Variables|Default|GetBackFlipbook)))
      (Variables|Default|SetActivationFlipbookLengthDown (Class|PaperFlipbookComponent|GetFlipbookLengthinFrames (Variables|Default|GetFrontFlipbook))))
    (:then_1
      (CallFunction|SetInitialFrames))
    (:then_2
      (if (not (Variables|Default|GetLoopMovement))
        (CallFunction|DeactivateAnimationLooping)))))

(fn ShowCorpse
  (Rendering|SetVisibility (Variables|Default|GetCorpse) true false))

(fn RotateCorpse
  (params (PrinceCharacter :type Prince%20Character%20Object%20Reference))
  (bind _rightwards (Default|IsRightwards PrinceCharacter))
  (if _rightwards
    _
    (else
      (Transformation|SetWorldRotation (Variables|Default|GetCorpse) "0,180.000000, 0" false false)))
  (return))

(fn HideDamageSignal
  (Rendering|SetVisibility (Variables|Default|GetDamageSignal) false false))

(fn ShowDamageSignal
  (Rendering|SetVisibility (Variables|Default|GetDamageSignal) true false))

(fn ReloadLevel
  (bind _returnvalue (Game|GetCurrentLevelName true))
  (Game|OpenLevel(byName) (Utilities|String|StringToName _returnvalue)))

(fn HideCorpse
  (Rendering|SetVisibility (Variables|Default|GetCorpse) false false))

(fn SetInitialFrames
  (bind _ground (Variables|Default|GetGround))
  (if (Variables|Default|GetHasBorder)
    (Rendering|Components|Sprite|SetSprite _ground (Variables|Default|GetGroundSprite))
    (else
      (Rendering|Components|Sprite|SetSprite _ground (Variables|Default|GetGroundNoBorderSprite)))))

(fn ForwardMovement
  (CallFunction|PlaySound (Variables|Default|GetActivationSound) (Variables|Default|GetAudio))
  (Components|Timeline|PlayfromStart (Variables|Default|GetBackFlipbook))
  (Components|Timeline|PlayfromStart (Variables|Default|GetFrontFlipbook)))

(fn ReverseMovement
  (Components|Timeline|ReversefromEnd (Variables|Default|GetBackFlipbook))
  (Components|Timeline|ReversefromEnd (Variables|Default|GetFrontFlipbook)))

(fn ActivateTrap
  (params (LoopAnimation :type Boolean))
  (bind _backflipbook (Variables|Default|GetBackFlipbook))
  (bind _frontflipbook (Variables|Default|GetFrontFlipbook))
  (CallFunction|PlaySound (Variables|Default|GetActivationSound) (Variables|Default|GetAudio))
  (Components|Timeline|SetLooping _backflipbook LoopAnimation)
  (Components|Timeline|PlayfromStart _backflipbook)
  (Components|Timeline|SetLooping _frontflipbook LoopAnimation)
  (Components|Timeline|PlayfromStart _frontflipbook))

(fn DeactivateAnimationLooping
  (Components|Timeline|SetLooping (Variables|Default|GetBackFlipbook) false)
  (Components|Timeline|SetLooping (Variables|Default|GetFrontFlipbook) false))

(fn SetGroundSprites
  (params (GroundBorderSprite :type Paper%20Sprite%20Object%20Reference) (GroundNoBorderSprite :type Paper%20Sprite%20Object%20Reference))
  (Utilities|FlowControl|Sequence
    (:then_0
      (Variables|Default|SetGroundSprite GroundBorderSprite))
    (:then_1
      (Variables|Default|SetGroundNoBorderSprite GroundNoBorderSprite))))

(fn InitTrapActivation
  (params (PotentialVictim :type Actor%20Object%20Reference))
  (Utilities|Casting|CastToPrinceCharacter PotentialVictim)
  (Variables|Default|SetCurrentState "NewEnumerator1")
  (CallFunction|TrapActivated))

(fn InitTrapDeactivation
  (params (PotentialVictim :type Actor%20Object%20Reference))
  (Utilities|Casting|CastToPrinceCharacter PotentialVictim)
  (Variables|Default|SetCurrentState "NewEnumerator4")
  (CallFunction|TrapDeactivated))