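; GenericSwitch is a base floor switch that is pressed while a PrinceCharacter overlaps its ActivationBox and released when the overlap ends.
; Activation swaps visibility to pushed center and occluder sprites, plays a sound and calls ActivateGate, a debug-print placeholder meant for overriding.
; Deactivation only restores the unpushed sprites.
; SetSpriteComponents picks sprite art from the HasBorder and InLeftEdge flags.
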(event OnComponentEndOverlap(ActivationBox)
  (params (OtherActor :type Actor%20Object%20Reference) (OtherComp :type Primitive%20Component%20Object%20Reference) (OtherBodyIndex :type Integer))
  ;[1 1 1] Activation and deactivation.
  (Utilities|Casting|CastToPrinceCharacter OtherActor)
  (if (Variables|Default|GetPushed?)
    (Variables|Default|SetPushed? false)
    (CallFunction|DeActivateSwitch)))

(event OnComponentBeginOverlap(ActivationBox)
  (params (OtherActor :type Actor%20Object%20Reference) (OtherComp :type Primitive%20Component%20Object%20Reference) (OtherBodyIndex :type Integer) (bFromSweep :type Boolean) (SweepResult :type Hit%20Result%20Structure%20%28by%20ref%29))
  ;[1 1 1] Activation and deactivation.
  (Utilities|Casting|CastToPrinceCharacter OtherActor)
  (if (not (Variables|Default|GetPushed?))
    (Variables|Default|SetPushed? true)
    (CallFunction|ActivateSwitch)))

(event EventSetSpriteComponents
  (bind _centersprite (Variables|Default|GetCenterSprite))
  (bind _pushedsprite (Variables|Default|GetPushedSprite))
  (bind _inleftedge_ (Variables|Default|GetInLeftEdge?))
  ;[1 1 1] Appearance initialization
  (Rendering|Components|Sprite|SetSprite (Variables|Default|GetOcluder) (Variables|Default|GetSwitchDeactivatedOcluder))
  ;;[1 1 1] Center sprite
  (if (Variables|Default|GetHasBorder?)
    (Rendering|Components|Sprite|SetSprite _centersprite (Variables|Default|GetSwitchDeactivatedBorderSprite))
    ;;[1 1 1] Pushed sprite
    (if _inleftedge_
      (Rendering|Components|Sprite|SetSprite _pushedsprite (Variables|Default|GetSwitchActivatedBorderLeftEdgeSprite))
      ;;[1 1 1] Ocluder
      (Rendering|Components|Sprite|SetSprite (Variables|Default|GetOcluder) (Variables|Default|GetSwitchDeactivatedOcluder) :!label _label)
      (Rendering|Components|Sprite|SetSprite (Variables|Default|GetOcluderPushed) (Variables|Default|GetSwitchActivatedOcluder))
      (else
        (Rendering|Components|Sprite|SetSprite _pushedsprite (Variables|Default|GetSwitchActivatedBorderSprite))))
    (else
      (Rendering|Components|Sprite|SetSprite _centersprite (Variables|Default|GetSwitchDeactivatedNoBorderSprite))
      (if _inleftedge_
        (Rendering|Components|Sprite|SetSprite _pushedsprite (Variables|Default|GetSwitchActivatedNoBorderLeftEdgeSprite))
        (goto _label)
        (else
          (Rendering|Components|Sprite|SetSprite _pushedsprite (Variables|Default|GetSwitchActivatedNoBorderSprite)))))))

(fn ConstructionScript
  (|CallParentFunction))

(fn PushSprite
  (Utilities|FlowControl|Sequence
    (:then_0
      (Rendering|SetVisibility (Variables|Default|GetCenterSprite) false false)
      (Utilities|FlowControl|Sequence
        (:then_0
          (Rendering|SetVisibility (Variables|Default|GetPushedSprite) true false))
        (:then_1
          (Rendering|SetVisibility (Variables|Default|GetOcluderPushed) true false))))
    (:then_1
      (Rendering|SetVisibility (Variables|Default|GetOcluder) false false))))

(fn UnPushSprite
  (Utilities|FlowControl|Sequence
    (:then_0
      (Rendering|SetVisibility (Variables|Default|GetCenterSprite) true false)
      (Utilities|FlowControl|Sequence
        (:then_0
          (Rendering|SetVisibility (Variables|Default|GetPushedSprite) false false))
        (:then_1
          (Rendering|SetVisibility (Variables|Default|GetOcluderPushed) false false))))
    (:then_1
      (Rendering|SetVisibility (Variables|Default|GetOcluder) true false))))

(fn ActivateSwitch
  (Utilities|FlowControl|Sequence
    (:then_0
      (CallFunction|PushSprite))
    (:then_1
      (CallFunction|PlaySound))
    (:then_2
      (CallFunction|ActivateGate))
    (:then_3
      (Variables|Default|SetPushed? true))))

(fn PlaySound
  (Audio|PlaySound2D "/Game/Sound/Effects/ground_switch_activated.ground_switch_activated"))

(fn ActivateGate
  ;[1 1 1] OVERRIDE THIS
  (Development|PrintString "Activating gate."))

(fn DeActivateSwitch
  (CallFunction|UnPushSprite))