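; PrincePlayerState holds the Prince's sword-possession flag and syncs it with the PrinceGameInstance.
; The construction script casts and caches the game instance, then reads PrinceHasSword from it.
; StoreState calls StorePlayerState, which writes the flag back to the game instance.
; The event graph has no logic.
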(event EventBeginPlay)

(event EventTick
  (params (DeltaSeconds :type Float%20%28single-precision%29)))

(fn ConstructionScript
  (bind _asprince_game_instance (Utilities|Casting|CastToPrinceGameInstance (Game|GetGameInstance)))
  (bind _output_get (Variables|Default|SetGameInstance _asprince_game_instance))
  (Variables|Default|SetPrinceHasSword (Default|GetPrinceHasSword _output_get)))

(fn StorePlayerState
  (Default|SetPrinceHasSword (Variables|Default|GetGameInstance) (Variables|Default|GetPrinceHasSword)))

(fn StoreState
  (Utilities|FlowControl|Sequence
    (:then_0
      (CallFunction|StorePlayerState))))