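; MediaLibrary is a set of helper functions for playing video and sound and toggling the player's HUD.
; ShowVideo adds an InterlevelScene widget textured with the video material, starts the sound and media player, and returns play status and duration.
; PlaySound restarts a supplied audio component with a new sound, and StopSound halts it.
; SetHudVisibility shows or hides the current HUD through the PrinceController.
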(fn ShowVideo
  (params (PlayerControllerInstance :type Player%20Controller%20Object%20Reference) (AudioPlayer :type Audio%20Component%20Object%20Reference%20%28by%20ref%29) (VideoSound :type Media%20Sound%20Wave%20Object%20Reference%20%28by%20ref%29) (VideoPlayer :type Media%20Player%20Object%20Reference) (VideoMaterial :type Material%20Object%20Reference))
  (bind _returnvalue (UserInterface|CreateWidget "/Game/UI/InterlevelScene.InterlevelScene_C" PlayerControllerInstance))
  (UserInterface|Viewport|AddtoViewport _returnvalue 0)
  (Class|Image|SetBrushfromMaterial (Variables|/Game/UI/InterlevelScene.InterlevelScene_C|GetSceneScreen _returnvalue) VideoMaterial)
  (Utilities|FlowControl|Sequence
    (:then_0
      (CallFunction|PlaySound VideoSound AudioPlayer))
    (:then_1
      (bind _returnvalue_2 (Media|MediaPlayer|Play VideoPlayer :!class /Script/MediaAssets.MediaPlayer))
      (return _returnvalue_2 (Media|MediaPlayer|GetDuration VideoPlayer)))))

(fn PlaySound
  (params (SoundToPlay :type Sound%20Wave%20Object%20Reference) (AudioComponent :type Audio%20Component%20Object%20Reference))
  (Audio|Components|Audio|Stop AudioComponent)
  (Audio|Components|Audio|SetSound AudioComponent SoundToPlay)
  (Audio|Components|Audio|Play AudioComponent 0.0))

(fn StopSound
  (params (AudioComponene :type Audio%20Component%20Object%20Reference))
  (Audio|Components|Audio|Stop AudioComponene))

(fn SetHudVisibility
  (params (Visible? :type Boolean))
  (bind _asprince_controller (Utilities|Casting|CastToPrinceController (Game|GetPlayerController 0)))
  (if Visible?
    (Widget|SetVisibility (Variables|/Game/Blueprints/PrinceController.PrinceController_C|GetCurrentHUD _asprince_controller) "Visible")
    (else
      (Widget|SetVisibility (Variables|/Game/Blueprints/PrinceController.PrinceController_C|GetCurrentHUD _asprince_controller) "Hidden"))))