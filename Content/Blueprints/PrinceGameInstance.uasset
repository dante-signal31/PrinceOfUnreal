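; Game instance for the Prince game that holds the player's life and remaining time.
; On Init it seeds the current time left, current maximum life and current life from configured totals and an initial life value.
; Getter and setter functions expose the current values, while the total maximum and initial life are exposed through getters only.
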(event EventInit
  (Utilities|FlowControl|Sequence
    (:then_0
      (Variables|Default|SetCurrentTimeLeft (Variables|Default|GetTotalMaximumTime)))
    (:then_1
      (Variables|Default|SetCurrentMaximumLife (Variables|Default|GetTotalMaximumLife)))
    (:then_2
      (Variables|Default|SetCurrentLife (Variables|Default|GetInitialLife)))))

(fn GetCurrentTimeLeft
  (return (Variables|Default|GetCurrentTimeLeft)))

(fn SetCurrentTimeLeft
  (params (CurrentTimeLeft :type Timespan%20Structure))
  (Variables|Default|SetCurrentTimeLeft CurrentTimeLeft))

(fn GetTotalMaximumLife
  (return (Variables|Default|GetTotalMaximumLife)))

(fn GetInitialLife
  (return (Variables|Default|GetInitialLife)))

(fn GetCurrentLife
  (return (Variables|Default|GetCurrentLife)))

(fn SetCurrentLife
  (params (CurrentLife :type Integer))
  (Variables|Default|SetCurrentLife CurrentLife))

(fn GetCurrentMaximumLife
  (return (Variables|Default|GetCurrentMaximumLife)))

(fn SetCurrentMaximumLife
  (params (CurrentMaximumLife :type Integer))
  (Variables|Default|SetCurrentMaximumLife CurrentMaximumLife))