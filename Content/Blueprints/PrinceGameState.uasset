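; Game state for the Prince game that runs the countdown timer and tracks the active level camera.
; Time left loads from PrinceGameInstance on BeginPlay, counts down on Tick unless paused, and is written back on EndPlay.
; Setting a camera switches the player's view target, refreshes that camera's trembling grounds and moves PrinceCharacter event bindings from the old camera to the new one.
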(event EventBeginPlay
  (Utilities|FlowControl|Sequence
    (:then_0
      (CallFunction|InitCurrentTimeLeft))))

(event EventTick
  (params (DeltaSeconds :type Float%20%28single-precision%29))
  (Utilities|FlowControl|Sequence
    (:then_0
      (if (not (Variables|Default|GetTimerPaused))
        (CallFunction|UpdateCurrentTimeLeft DeltaSeconds)))))

(event EventEndPlay
  (params (EndPlayReason :type EEndPlayReason%20Enum :default "Destroyed"))
  (Utilities|FlowControl|Sequence
    (:then_0
      (CallFunction|StoreCurrentTimeLeft))))

(fn ConstructionScript
  (bind _asprince_game_instance (Utilities|Casting|CastToPrinceGameInstance (Game|GetGameInstance)))
  (Variables|Default|SetGameInstance _asprince_game_instance))

(fn GetCurrentTimeLeft
  (return (Variables|Default|GetCurrentTimeLeft)))

(fn SetCurrentTimeLeft
  (params (CurrentTimeLeft :type Timespan%20Structure))
  (Variables|Default|SetCurrentTimeLeft CurrentTimeLeft))

(fn InitCurrentTimeLeft
  (Variables|Default|SetCurrentTimeLeft (Default|GetCurrentTimeLeft (Variables|Default|GetGameInstance)))
  (return))

(fn UpdateCurrentTimeLeft
  (params (Seconds :type Float%20%28single-precision%29))
  (Variables|Default|SetCurrentTimeLeft (- (Variables|Default|GetCurrentTimeLeft) (Math|Timespan|FromSeconds Seconds)))
  (return))

(fn StoreCurrentTimeLeft
  (bind _asprince_game_instance (Utilities|Casting|CastToPrinceGameInstance (Game|GetGameInstance))
    (:then
      (Default|SetCurrentTimeLeft _asprince_game_instance (Variables|Default|GetCurrentTimeLeft)))
    (:CastFailed
      _))
  (return))

(fn SetCurrentLevelCamera
  (params (CurrentCamera :type Level%20Camera%20Object%20Reference))
  (bind _output_get (LocalVariables|SetOldCamera (Variables|Default|GetCurrentCamera)))
  (bind _output_get_2 (Variables|Default|SetCurrentCamera CurrentCamera))
  (bind _asprince_character (Utilities|Casting|CastToPrinceCharacter (Game|GetPlayerCharacter 0)))
  (Utilities|FlowControl|Sequence
    (:then_1
      ;[1 1 1] Update view to new camera.
      (Game|Player|SetViewTargetwithBlend (Game|GetPlayerController 0) _output_get_2 0.0 "VTBlend_Linear" 0.0 false))
    (:then_2
      ;[1 1 1] Refresh trembling grounds list.
      (Default|LocateTremblingGrounds _output_get_2)
      (Utilities|FlowControl|Sequence
        (:then_0
          ;[1 1 1] Update binding of interested actors in area to PrinceCharacter events.
          (Default|BindCharacter _output_get_2 _asprince_character))
        (:then_1
          (if (!= _output_get 0)
            (Default|UnbindCharacter _output_get _asprince_character)))))))

(fn GetCurrentLevelCamera
  (return (Variables|Default|GetCurrentCamera)))

(fn PauseTimer
  (Variables|Default|SetTimerPaused true))

(fn ResumeTimer
  (Variables|Default|SetTimerPaused false))