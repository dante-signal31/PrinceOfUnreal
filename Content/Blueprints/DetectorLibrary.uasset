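; Blueprint library with a detection helper that returns the actors of a given class located inside an area, described as the camera bounding box.
; GetInstancesInArea derives X and Z limits from the area component's bounds, then filters every actor of that class against them.
; The test is 2D on the XZ plane: it ignores Y and compares actor locations only, without using collision overlaps or actor extents.
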(fn GetInstancesinArea
  (params (Area :type Box%20Component%20Object%20Reference) (ClassToLookFor :type Actor%20Class%20Reference))
  (bind (_origin _boxextent) (Collision|GetComponentBounds Area))
  (bind (_x _y _z) (Math|Vector|BreakVector _origin))
  (bind (_x_2 _y_2 _z_2) (Math|Vector|BreakVector _boxextent))
  ;[1 1 1] Calculate 2D dimensions of camera bounding box.
  (LocalVariables|SetMinimumX (- _x _x_2))
  (LocalVariables|SetMaximumX (+ _x _x_2))
  (LocalVariables|SetMinimumZ (- _z _z_2))
  (LocalVariables|SetMaximumZ (+ _z _z_2))
  ;[1 1 1] Include in array every found objet that is inside camera bounding box.
  (bind _outactors (Actor|GetAllActorsOfClass 0 ClassToLookFor))
  (for _array_element _outactors
    (if (and (and (>= (.X (Math|Vector|BreakVector (Transformation|GetActorLocation _array_element))) (LocalVariables|GetMinimumX)) (<= (.X (Math|Vector|BreakVector (Transformation|GetActorLocation _array_element))) (LocalVariables|GetMaximumX))) (and (>= (.Z (Math|Vector|BreakVector (Transformation|GetActorLocation _array_element))) (LocalVariables|GetMinimumZ)) (<= (.Z (Math|Vector|BreakVector (Transformation|GetActorLocation _array_element))) (LocalVariables|GetMaximumZ))))
      (Utilities|Array|Add (LocalVariables|GetActorArrayToReturn) _array_element)))
  (return (LocalVariables|GetActorArrayToReturn)))