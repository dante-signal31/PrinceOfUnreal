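; Trigger gate that switches between two fixed cameras, left/right or up/down per HorizontalChanger, as the PrinceCharacter crosses it.
; On begin overlap, it compares the Prince's X or Z position to its own and points player 0's view at the opposite side's camera.
; On end overlap, it rechecks the exit side and corrects any mismatch through PrinceGameState's SetCurrentLevelCamera, covering a Prince who backs out.
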(event EventActorBeginOverlap
  (params (OtherActor :type Actor%20Object%20Reference))
  ;[1 1 1] Set new camera.
  (bind _asprince_character (Utilities|Casting|CastToPrinceCharacter OtherActor))
  (bind _output_get (Variables|Default|SetCurrentCamera (select (Variables|Default|GetHorizontalChanger) (select (.IsRight? (CallFunction|GetPrinceLocationRelativetoGate _asprince_character)) (Variables|Default|GetLeftCamera) (Variables|Default|GetRightCamera)) (select (.IsUp? (CallFunction|GetPrinceLocationRelativetoGate _asprince_character)) (Variables|Default|GetDownCamera) (Variables|Default|GetUpCamera)))))
  (Game|Player|SetViewTargetwithBlend (Game|GetPlayerController 0) _output_get 0.0 "VTBlend_Linear" 0.0 false))

(event Collision|EventActorEndOverlap
  (params (OtherActor :type Actor%20Object%20Reference))
  ;[1 1 1] Check set camera is still correct.
  (bind _asprince_character (Utilities|Casting|CastToPrinceCharacter OtherActor))
  (if (not (== (Variables|Default|GetCurrentCamera) (select (Variables|Default|GetHorizontalChanger) (select (.IsRight? (CallFunction|GetPrinceLocationRelativetoGate _asprince_character)) (Variables|Default|GetRightCamera) (Variables|Default|GetLeftCamera)) (select (.IsUp? (CallFunction|GetPrinceLocationRelativetoGate _asprince_character)) (Variables|Default|GetUpCamera) (Variables|Default|GetDownCamera)))))
    (bind _output_get (Variables|Default|SetCurrentCamera (select (Variables|Default|GetHorizontalChanger) (select (.IsRight? (CallFunction|GetPrinceLocationRelativetoGate _asprince_character)) (Variables|Default|GetRightCamera) (Variables|Default|GetLeftCamera)) (select (.IsUp? (CallFunction|GetPrinceLocationRelativetoGate _asprince_character)) (Variables|Default|GetUpCamera) (Variables|Default|GetDownCamera)))))
    (bind _asprince_game_state (Utilities|Casting|CastToPrinceGameState (Game|GetGameState)))
    (Default|SetCurrentLevelCamera _asprince_game_state _output_get)))

(fn ConstructionScript)

(fn GetPrinceLocationRelativetoGate
  (params (PrinceActor :type Actor%20Object%20Reference))
  (bind _returnvalue (Transformation|GetActorLocation PrinceActor))
  (bind _returnvalue_2 (Transformation|GetActorLocation))
  (bind _returnvalue_3 (- _returnvalue _returnvalue_2))
  (bind (_x _y _z) (Math|Vector|BreakVector _returnvalue_3))
  (return (> _x 0.0) (> _z 0.0)))