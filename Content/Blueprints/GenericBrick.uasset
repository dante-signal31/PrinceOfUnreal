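; GenericBrick is a base Blueprint for Paper2D bricks that can repeat into a grid and expose left and right ledge-grab points.
; Its construction script calls SetSpriteComponents, an empty hook for child Blueprints, then records the center sprite's child sprites with their relative transforms.
; It then adds copies of the center and satellite sprites at set spacing, extending along X and Z in directions chosen by Rightwards and Downwards.
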(fn ConstructionScript
  (bind _centersprite (Variables|Default|GetCenterSprite))
  (Utilities|FlowControl|Sequence
    (:then_0
      ;[1 1 1] To be overriden in children blueprints
      (CallFunction|SetSpriteComponents))
    (:then_1
      ;[1 1 1] Replicate appearance if you want to place a brick array.
      (bind _children (CallFunction|GetChildrenSprites _centersprite))
      (Variables|Default|SetOriginalSpriteComponents _children))
    (:then_2
      (CallFunction|CreateGrid (Variables|Default|GetAmountX) (Variables|Default|GetAmountZ) _centersprite))))

(fn SetSpriteComponents
  ;[1 1 1] This function should be overriden by children blueprints
)

(fn GetChildrenSprites
  (params (RootSprite :type Paper%20Sprite%20Component%20Object%20Reference))
  (for _array_element (Components|GetChildrenComponents RootSprite false)
    ;[1 1 1] Register satellite sprite component location relative to root sprite.
    (bind _aspaper_sprite_component (Utilities|Casting|CastToPaperSpriteComponent _array_element))
    (Utilities|Array|Add (LocalVariables|Get_Children) (Utilities|Struct|MakeSpriteComponent (Variables|/Script/Paper2D.PaperSpriteComponent|GetSourceSprite _aspaper_sprite_component) (Transformation|GetRelativeTransform _aspaper_sprite_component))))
  (return (LocalVariables|Get_Children)))

(fn CreateGrid
  (params (AmountX :type Integer) (AmountZ :type Integer) (RootSprite :type Paper%20Sprite%20Component%20Object%20Reference))
  ;[1 1 1] Row creation loop
  (if (> AmountX 0)
    (for _index (range 0 (- AmountX 1))
      ;[1 1 1] Column creation loop
      (for _index_2 (range 0 AmountZ)
        (CallFunction|CreateBrickCopy _index _index_2 RootSprite)))
    (elif (> AmountZ 0)
      (for _index_3 (range 0 AmountZ)
        (CallFunction|CreateBrickCopy _index _index_3 RootSprite)))))

(fn CreateBrickCopy
  (params (IndexX :type Integer) (IndexZ :type Integer) (RootSprite :type Paper%20Sprite%20Component%20Object%20Reference))
  (bind _copycenterrelativelocation (CallFunction|GetCopyCenter IndexX IndexZ RootSprite))
  (Utilities|FlowControl|Sequence
    (:then_0
      ;[1 1 1] Copy center component
      (bind _returnvalue (AddComponent|AddPaperSpriteComponent false _copycenterrelativelocation))
      (Rendering|Components|Sprite|SetSprite _returnvalue (Variables|/Script/Paper2D.PaperSpriteComponent|GetSourceSprite RootSprite)))
    (:then_1
      (CallFunction|CopyChildrenComponents _copycenterrelativelocation))))

(fn GetCopyCenter
  (params (IndexX :type Integer) (IndexZ :type Integer) (RootSprite :type Paper%20Sprite%20Component%20Object%20Reference))
  (bind (_scalarx _scalarz) (CallFunction|GetRepetitionScalars))
  (bind (_dimensionx _dimensionz) (CallFunction|GetCloningDimensions RootSprite))
  (return (Math|Conversions|ToTransform(Vector) (Math|Vector|MakeVector (* (* IndexX _scalarx) _dimensionx) 0.0 (* (* IndexZ _scalarz) _dimensionz)))))

(fn GetRepetitionScalars
  (Utilities|FlowControl|Sequence
    (:then_0
      (if (Variables|Default|GetRightwards)
        (LocalVariables|SetX 1)
        (else
          (LocalVariables|SetX -1))))
    (:then_1
      (if (Variables|Default|GetDownwards)
        (LocalVariables|SetZ -1)
        (else
          (LocalVariables|SetZ 1))))
    (:then_2
      (return (LocalVariables|GetX) (LocalVariables|GetZ)))))

(fn GetCloningDimensions
  (params (SpriteComponent :type Paper%20Sprite%20Component%20Object%20Reference))
  (return (Variables|Default|GetCloneDistanceX) (Variables|Default|GetCloneDistanceZ)))

(fn CopyChildrenComponents
  (params (RootSpriteTransform :type Transform))
  (for _array_element (Variables|Default|GetOriginalSpriteComponents)
    ;[1 1 1] Draw child component of brick copy
    (bind _returnvalue (AddComponent|AddPaperSpriteComponent false (Math|Transform|MakeTransform (+ (.Location (Math|Transform|BreakTransform (.RelativeCoordinates (Utilities|Struct|BreakSpriteComponent _array_element)))) (.Location (Math|Transform|BreakTransform RootSpriteTransform))) (.Rotation (Math|Transform|BreakTransform (.RelativeCoordinates (Utilities|Struct|BreakSpriteComponent _array_element)))) (.Scale (Math|Transform|BreakTransform (.RelativeCoordinates (Utilities|Struct|BreakSpriteComponent _array_element)))))))
    (Rendering|Components|Sprite|SetSprite _returnvalue (.Sprite (Utilities|Struct|BreakSpriteComponent _array_element))))
  (return))

(fn GetGrabingPoint
  (params (ReturnRightPoint? :type Boolean))
  (if ReturnRightPoint?
    (return (Transformation|GetWorldLocation (Variables|Default|GetLedgeGrabingPointRight)))
    (else
      (return (Transformation|GetWorldLocation (Variables|Default|GetLedgeGrabingPointLeft))))))