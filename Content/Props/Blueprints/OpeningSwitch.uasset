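; Switch prop Blueprint that opens a gate when pushed and activates that gate's open timer when released.
; It overrides the parent switch's activate and deactivate events, sending the actions to the gate as interface messages.
; Sprite setup extends the parent's, swapping the center sprite for bordered or borderless left-edge variants when the switch sits on a left edge.
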(event EventDeactivateGate
  (params (Gate :type Actor%20Object%20Reference))
  ;[1 1 1] Unpush switch
  (Class|GateInterface|ActivateOpenTimer(Message) Gate))

(event EventActivateGate
  (params (Gate :type Actor%20Object%20Reference))
  ;[1 1 1] Push switch
  (Class|GateInterface|OpenGate(Message) Gate))

(event EventSetSpriteComponents
  (bind _centersprite (Variables|Default|GetCenterSprite))
  (|CallParentFunction)
  ;[1 1 1] Visual setup.
  ;;[1 1 1] False case implemented in parent function.
  (if (Variables|Default|GetInLeftEdge?)
    ;;[1 1 1] Center sprite
    (if (Variables|Default|GetHasBorder?)
      (Rendering|Components|Sprite|SetSprite _centersprite (Variables|Default|GetSwitchDeactivatedBorderLeftEdge))
      (else
        (Rendering|Components|Sprite|SetSprite _centersprite (Variables|Default|GetSwitchDeactivatedNoBorderLeftEdge))))))

(fn ConstructionScript
  (|CallParentFunction))