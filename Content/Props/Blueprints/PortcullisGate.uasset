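; Portcullis gate prop that raises and lowers its iron curtain with matching sounds, plus an optional ground-border sprite.
; Open, slow-close and fast-close events set a state machine that Tick uses to move the curtain between clamped height bounds.
; The construction script derives speeds from elevation height and travel times, then applies the initial state.
; When autoclose is enabled and its timer activated, the open gate closes slowly after a timeout.
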(event EventActivateOpenTimer
  ;[1 1 1] If autoclose then start countdown to close
  (Variables|Default|SetOpenTimerActivated true))

(event EventTick
  (params (DeltaSeconds :type Float%20%28single-precision%29))
  (bind _audio (Variables|Default|GetAudio))
  (switch Utilities|FlowControl|Switch|SwitchonGateStates (Variables|Default|GetState)
    (:NewEnumerator1
      ;[1 1 1] Animations
      (CallFunction|MovePortcullis DeltaSeconds (Variables|Default|GetOpeningSpeed) false "NewEnumerator3")
      ;[1 1 1] Stop current sound if movement already ended
      (switch Utilities|FlowControl|Switch|SwitchonGateStates (Variables|Default|GetState)
        (:NewEnumerator3
          (CallFunction|StopSound _audio))))
    (:NewEnumerator3
      ;[1 1 1] Autoclose timer
      (CallFunction|UpdateOpenTimer DeltaSeconds)
      (bind _timeoutreached (CallFunction|OpenTimeoutReached?))
      (if _timeoutreached
        (CallFunction|StopOpenTimer)
        (CallFunction|CloseGateSlow)))
    (:NewEnumerator2
      (CallFunction|MovePortcullis DeltaSeconds (Variables|Default|GetSlowClosingSpeed) true "NewEnumerator0")
      (switch Utilities|FlowControl|Switch|SwitchonGateStates (Variables|Default|GetState)
        (:NewEnumerator0
          (CallFunction|StopSound _audio))))
    (:NewEnumerator4
      (CallFunction|MovePortcullis DeltaSeconds (Variables|Default|GetFastClosingSpeed) true "NewEnumerator0")
      ;[1 1 1] Closing fast bang
      (switch Utilities|FlowControl|Switch|SwitchonGateStates (Variables|Default|GetState)
        (:NewEnumerator0
          (CallFunction|PlaySound "/Game/Sound/Effects/portcullis_closing_fast.portcullis_closing_fast" (Variables|Default|GetAudio)))))))

(event EventOpenGate
  ;[1 1 1] Open
  (switch Utilities|FlowControl|Switch|SwitchonGateStates (Variables|Default|GetState)
    (:NewEnumerator0
      _)
    (:NewEnumerator2
      _)
    (:NewEnumerator4
      _))
  (Variables|Default|SetState "NewEnumerator1")
  (CallFunction|PlaySound "/Game/Sound/Effects/portcullis_opening.portcullis_opening" (Variables|Default|GetAudio)))

(event EventSetSpriteComponents
  ;[1 1 1] Appearance customization
  (CallFunction|SetGroundBorder))

(event EventCloseGateSlow
  ;[1 1 1] Close slowly
  (switch Utilities|FlowControl|Switch|SwitchonGateStates (Variables|Default|GetState)
    (:NewEnumerator3
      (Variables|Default|SetState "NewEnumerator2")
      (CallFunction|PlaySound "/Game/Sound/Effects/portcullis_closing_slowly.portcullis_closing_slowly" (Variables|Default|GetAudio)))))

(event EventCloseGateFast
  ;[1 1 1] Close fast
  (switch Utilities|FlowControl|Switch|SwitchonGateStates (Variables|Default|GetState)
    (:NewEnumerator1
      _)
    (:NewEnumerator3
      _)
    (:NewEnumerator2
      _))
  (Variables|Default|SetState "NewEnumerator4"))

(fn ConstructionScript
  (|CallParentFunction)
  (Utilities|FlowControl|Sequence
    (:then_0
      (CallFunction|InitMovementParameters))
    (:then_1
      (CallFunction|InitBounds))
    (:then_2
      (CallFunction|SetInitialState))))

(fn InitMovementParameters
  (bind _elevationheight (Variables|Default|GetElevationHeight))
  (bind _returnvalue (Math|Conversions|ToFloat(Integer) _elevationheight))
  (Utilities|FlowControl|Sequence
    (:then_0
      (Variables|Default|SetOpeningSpeed (/ _returnvalue (Variables|Default|GetOpeningTime))))
    (:then_1
      (Variables|Default|SetSlowClosingSpeed (/ _returnvalue (Variables|Default|GetSlowClosingTime))))
    (:then_2
      (Variables|Default|SetFastClosingSpeed (/ _returnvalue (Variables|Default|GetFastClosingTime))))))

(fn InitBounds
  (bind _ironcurtainleft (Variables|Default|GetIronCurtainLeft))
  (bind _relativelocation (Variables|/Script/Engine.SceneComponent|GetRelativeLocation _ironcurtainleft))
  (Variables|Default|SetInitialElevation (Math|Float|Truncate (.z _relativelocation)))
  (Variables|Default|SetMaximumElevation (Math|Float|Truncate (+ (.z _relativelocation) (Math|Conversions|ToFloat(Integer) (Variables|Default|GetElevationHeight))))))

(fn MovePortcullis
  (params (Delta :type Float%20%28single-precision%29) (Speed :type Float%20%28single-precision%29) (Downwards? :type Boolean) (NewStateOnBoundReached :type GateStates%20Enum))
  (if Downwards?
    (if (CallFunction|OverMinimumElevation?)
      ;[1 1 1] Inside threshold: keep moving
      (Transformation|SetRelativeLocation (Variables|Default|GetIronCurtainLeft) (CallFunction|GetPorcullisAdvance Delta Speed Downwards?) false true :!label _label)
      (else
        ;[1 1 1] Threshold reached: movement finished
        (Variables|Default|SetState NewStateOnBoundReached)))
    (elif (CallFunction|UnderMaximumElevation?)
      (goto _label)
      (else
        (Variables|Default|SetState NewStateOnBoundReached))))
  (return))

(fn GetPorcullisAdvance
  (params (Delta :type Float%20%28single-precision%29) (Speed :type Float%20%28single-precision%29) (Downwards? :type Boolean))
  (bind _returnvalue (* Delta Speed))
  (bind _ironcurtainleft (Variables|Default|GetIronCurtainLeft))
  (bind _relativelocation (Variables|/Script/Engine.SceneComponent|GetRelativeLocation _ironcurtainleft))
  (if Downwards?
    (LocalVariables|SetNewZLocationUnclamped (- (.z _relativelocation) _returnvalue))
    (else
      (LocalVariables|SetNewZLocationUnclamped (+ (.z _relativelocation) _returnvalue))))
  (return (Math|Vector|MakeVector (.x _relativelocation) (.y _relativelocation) (Math|Float|Clamp(Float) (LocalVariables|GetNewZLocationUnclamped) (Math|Conversions|ToFloat(Integer) (Variables|Default|GetInitialElevation)) (Math|Conversions|ToFloat(Integer) (Variables|Default|GetMaximumElevation))))))

(fn UnderMaximumElevation?
  (return (< (.z (Variables|/Script/Engine.SceneComponent|GetRelativeLocation (Variables|Default|GetIronCurtainLeft))) (Math|Conversions|ToFloat(Integer) (Variables|Default|GetMaximumElevation)))))

(fn OverMinimumElevation?
  (return (> (.z (Variables|/Script/Engine.SceneComponent|GetRelativeLocation (Variables|Default|GetIronCurtainLeft))) (Math|Conversions|ToFloat(Integer) (Variables|Default|GetInitialElevation)))))

(fn StartOpenTimer
  (Variables|Default|SetOpenTimerActivated true)
  (Variables|Default|SetOpenTimer 0.0))

(fn StopOpenTimer
  (Variables|Default|SetOpenTimerActivated false)
  (Variables|Default|SetOpenTimer 0.0))

(fn OpenTimeoutReached?
  (return (and (Variables|Default|GetAutoclose?) (>= (Variables|Default|GetOpenTimer) (Variables|Default|GetOpenTimeout)))))

(fn UpdateOpenTimer
  (params (Delta :type Float%20%28single-precision%29))
  (if (and (Variables|Default|GetAutoclose?) (Variables|Default|GetOpenTimerActivated))
    (Variables|Default|SetOpenTimer (+ (Variables|Default|GetOpenTimer) Delta))))

(fn ActivateOpenTimer?
  (return (and (Variables|Default|GetAutoclose?) (not (Variables|Default|GetOpenTimerActivated)))))

(fn PlaySound
  (params (Sound%20to%20play :type Sound%20Base%20Object%20Reference))
  (bind _audio (Variables|Default|GetAudio))
  (Audio|Components|Audio|Stop _audio)
  (Audio|Components|Audio|SetSound _audio Sound%20to%20play)
  (Audio|Components|Audio|Play _audio 0.0))

(fn SetGroundBorder
  (bind _centersprite (Variables|Default|GetCenterSprite))
  (if (Variables|Default|GetHasBorder)
    (Rendering|Components|Sprite|SetSprite _centersprite (Variables|Default|GetGroundBorderSprite))
    (else
      (Rendering|Components|Sprite|SetSprite _centersprite (Variables|Default|GetGroundNoBorderSprite))))
  (return))

(fn SetOpenPosition
  (bind _ironcurtainleft (Variables|Default|GetIronCurtainLeft))
  (bind _relativelocation (Variables|/Script/Engine.SceneComponent|GetRelativeLocation _ironcurtainleft))
  (Transformation|SetRelativeLocation _ironcurtainleft (Math|Vector|MakeVector (.x _relativelocation) (.y _relativelocation) (+ (.z _relativelocation) (Math|Conversions|ToFloat(Integer) (Variables|Default|GetElevationHeight)))) false true)
  (return))

(fn SetInitialState
  (bind _output_get (Variables|Default|SetState (Variables|Default|GetInitialState)))
  (switch Utilities|FlowControl|Switch|SwitchonGateStates _output_get
    (:NewEnumerator0
      _)
    (:NewEnumerator1
      (CallFunction|SetOpenPosition :!label _label))
    (:NewEnumerator3
      (goto _label))
    (:NewEnumerator2
      (goto _label))
    (:NewEnumerator4
      (goto _label)))
  (return))