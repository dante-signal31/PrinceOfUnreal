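; Wall brick prop built from Paper2D sprite layers for ground, cut wall, things over ground and an occluder.
; SetSpriteComponents applies the ground, border, cut-wall and overlay settings by swapping sprites and toggling ground visibility.
; ShowGarbage adds debris when falling ground crashes on it, and ShowBorder updates the edge when neighboring floor falls.
; Both ground-border and overlay logic write the occluder sprite, so the later call wins.
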(event EventShowGarbage
  ;[1 1 1] Dropping ground crashed against this brick.
  (CallFunction|PlaceThingsOverGround "NewEnumerator1"))

(event EventBeginPlay)

(event EventActorBeginOverlap
  (params (OtherActor :type Actor%20Object%20Reference)))

(event EventSetSpriteComponents
  ;[1 1 1] Configure sprites to be shown.
  (CallFunction|SetGround (Variables|Default|GetHasGround) (Variables|Default|GetHasBorder))
  (CallFunction|SetCutwall (Variables|Default|GetHasCutWall))
  (CallFunction|PlaceThingsOverGround (Variables|Default|GetThingToPlaceOverGround)))

(event EventShowBorder
  (params (show? :type Boolean))
  ;[1 1 1] Floor next to this brick has fallen and we need to show border.
  (bind _output_get (Variables|Default|SetHasBorder show?))
  (CallFunction|SetGround (Variables|Default|GetHasGround) _output_get))

(fn ConstructionScript
  (|CallParentFunction))

(fn PlaceThingsOverGround
  (params (ThingToPlace :type ThingsOverGround%20Enum))
  (bind _thingsoverground (Variables|Default|GetThingsOverGround))
  (bind _ocluder (Variables|Default|GetOcluder))
  (switch Utilities|FlowControl|Switch|SwitchonThingsOverGround ThingToPlace
    (:NewEnumerator0
      (Rendering|Components|Sprite|SetSprite _thingsoverground 0)
      (Rendering|Components|Sprite|SetSprite _ocluder "/Game/Props/Sprites/Dungeon/_Ocluder_ground_Sprite_normalized._Ocluder_ground_Sprite_normalized"))
    (:NewEnumerator1
      (Rendering|Components|Sprite|SetSprite _thingsoverground "/Game/Props/Sprites/Dungeon/_Ground_garbage_normalized_Sprite._Ground_garbage_normalized_Sprite")
      (Rendering|Components|Sprite|SetSprite _ocluder "/Game/Props/Sprites/Dungeon/_Ground_garbage_occluder_n_Sprite._Ground_garbage_occluder_n_Sprite"))
    (:NewEnumerator2
      (Rendering|Components|Sprite|SetSprite _thingsoverground "/Game/Props/Sprites/Dungeon/_Ground_bones_normalized_Sprite._Ground_bones_normalized_Sprite")
      (Rendering|Components|Sprite|SetSprite _ocluder "/Game/Props/Sprites/Dungeon/_Ground_bones_ocluder_n_Sprite._Ground_bones_ocluder_n_Sprite")))
  (return))

(fn SetGround
  (params (showGround? :type Boolean) (showBorder? :type Boolean))
  (bind _ground (Variables|Default|GetGround))
  (Rendering|SetVisibility (Variables|Default|GetGround) showGround? true)
  (if showBorder?
    (Rendering|Components|Sprite|SetSprite _ground (Variables|Default|GetGroundBorderSprite))
    (Rendering|Components|Sprite|SetSprite (Variables|Default|GetOcluder) (Variables|Default|GetOcluderSprite))
    (else
      (Rendering|Components|Sprite|SetSprite _ground (Variables|Default|GetGroundNoBorderSprite)))))

(fn SetCutwall
  (params (showCutwall? :type Boolean))
  (bind _cutwall (Variables|Default|GetCutwall))
  (if showCutwall?
    (Rendering|Components|Sprite|SetSprite _cutwall (Variables|Default|GetCutWallSprite))
    (else
      (Rendering|Components|Sprite|SetSprite _cutwall 0))))

(fn BorderShown
  (return (Variables|Default|GetHasBorder)))