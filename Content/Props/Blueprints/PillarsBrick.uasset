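; PillarsBrick is a brick pillar prop built from Paper2D sprite components, with variants with and without a ground border.
; Its SetSpriteComponents event checks HasGroundBorder and assigns the matching sprites to the back pillar and to the center component, which shows the front pillar.
; The construction script only runs the parent's, and nothing in this graph calls SetSpriteComponents.
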(event EventBeginPlay)

(event EventActorBeginOverlap
  (params (OtherActor :type Actor%20Object%20Reference)))

(event EventSetSpriteComponents
  (bind _backpillar (Variables|Default|GetBackPillar))
  (bind _centersprite (Variables|Default|GetCenterSprite))
  (if (Variables|Default|GetHasGroundBorder)
    (Rendering|Components|Sprite|SetSprite _backpillar (Variables|Default|GetBackPillarBorderSprite))
    (Rendering|Components|Sprite|SetSprite _centersprite (Variables|Default|GetFrontPillarBorderSprite))
    (else
      (Rendering|Components|Sprite|SetSprite _backpillar (Variables|Default|GetBackPillarNoBorderSprite))
      (Rendering|Components|Sprite|SetSprite _centersprite (Variables|Default|GetFrontPillarNoBorderSprite)))))

(fn ConstructionScript
  (|CallParentFunction))