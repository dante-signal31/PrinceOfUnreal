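; Spike trap prop, built on a parent trap, that rises on activation and kills the Prince on contact.
; Back and front flipbooks animate the spikes, with back-flipbook finish events setting Active or Inactive state.
; The killing zone kills only in certain running, turning, jump-landing or falling states, then plays death music and reloads the level.
; The construction script sets sounds and ground sprites, and matches spike and corpse visuals to the current state.
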(event OnComponentBeginOverlap(KillingZone)
  (params (OtherActor :type Actor%20Object%20Reference) (OtherComp :type Primitive%20Component%20Object%20Reference) (OtherBodyIndex :type Integer) (bFromSweep :type Boolean) (SweepResult :type Hit%20Result%20Structure%20%28by%20ref%29))
  (bind _audio (Variables|Default|GetAudio))
  ;[1 1 1] Into the killing zone
  (bind _asprince_character (Utilities|Casting|CastToPrinceCharacter OtherActor))
  (switch Utilities|FlowControl|Switch|SwitchonPrinceStates (Default|GetState _asprince_character)
    (:NewEnumerator1
      _)
    (:NewEnumerator2
      _)
    (:NewEnumerator3
      _)
    (:NewEnumerator22
      _)
    (:NewEnumerator16
      (Variables|Default|SetPlayChaftSound? true :!label _label))
    (:NewEnumerator6
      (goto _label))
    (:NewEnumerator12
      _))
  (Utilities|KillPrince _asprince_character self (Variables|Default|GetPlayChaftSound?)
    (:Exit
      (Utilities|FlowControl|Delay 2.0)
      ;;[0.3414 0.3421 1] Restart level
      (CallFunction|PlaySound (Variables|Default|GetDeathMusic) _audio)
      (EventDispatchers|BindEventtoOnAudioFinished _audio (delegate Custom|RestartLevel)))))

(event Custom|SpikesDeactivated
  ;[1 1 1] Spikes deactivation
  (CallFunction|HideSpikes)
  (Variables|Default|SetCurrentState "NewEnumerator0")
  (EventDispatchers|UnbindEventfromOnFinishedPlaying (Variables|Default|GetBackFlipbook) (delegate Custom|SpikesDeactivated)))

(event Custom|SpikesFullyActivated
  ;[1 1 1] Spikes activation
  (Variables|Default|SetCurrentState "NewEnumerator2")
  (EventDispatchers|UnbindEventfromOnFinishedPlaying (Variables|Default|GetBackFlipbook) (delegate Custom|SpikesFullyActivated)))

(event Custom|RestartLevel
  ;[1 1 1] Into the killing zone
  ;;[0.3414 0.3421 1] Restart level
  (EventDispatchers|UnbindEventfromOnAudioFinished (Variables|Default|GetAudio) (delegate Custom|RestartLevel))
  (CallFunction|ReloadLevel))

(event Custom|TrapDeactivated
  (bind _backflipbook (Variables|Default|GetBackFlipbook))
  ;[1 1 1] Spikes deactivation
  (EventDispatchers|BindEventtoOnFinishedPlaying _backflipbook (delegate Custom|SpikesDeactivated))
  (Components|Timeline|ReversefromEnd _backflipbook)
  (Components|Timeline|ReversefromEnd (Variables|Default|GetFrontFlipbook)))

(event EventTrapActivated
  ;[1 1 1] Spikes activation
  (EventDispatchers|BindEventtoOnFinishedPlaying (Variables|Default|GetBackFlipbook) (delegate Custom|SpikesFullyActivated))
  (CallFunction|ShowSpikes)
  (CallFunction|ActivateTrap false))

(fn ConstructionScript
  (Utilities|FlowControl|Sequence
    (:then_0
      ;[1 1 1] Setup
      (Variables|Default|SetActivationSound (Variables|Default|GetSpikesActivationSound))
      (Variables|Default|SetChaftSound (Variables|Default|GetSpikesChaftSound)))
    (:then_1
      (Variables|Default|SetCorpseSprite (Variables|Default|GetCorpseSprite)))
    (:then_2
      (CallFunction|SetGroundSprites (Variables|Default|GetSpikesTrapGroundSprite) (Variables|Default|GetSpikesTrapGroundNoBorderSprite))
      (|CallParentFunction)
      ;[1 1 1] Behavior.
      (switch Utilities|FlowControl|Switch|SwitchonTrapStates (Variables|Default|GetCurrentState)
        (:NewEnumerator0
          (CallFunction|HideSpikes :!label _label)
          (CallFunction|HideCorpse :!label _label_2)
          (CallFunction|HideDamageSignal))
        (:NewEnumerator1
          (goto _label))
        (:NewEnumerator2
          (CallFunction|SetSpikesUp :!label _label_3)
          (goto _label_2))
        (:NewEnumerator3
          (CallFunction|SetSpikesUp)
          (CallFunction|ShowCorpse))
        (:NewEnumerator4
          (goto _label_3))))))

(fn HideSpikes
  (bind _backflipbook (Variables|Default|GetBackFlipbook))
  (bind _frontflipbook (Variables|Default|GetFrontFlipbook))
  (Audio|Components|Audio|Stop _backflipbook)
  (Rendering|SetVisibility _backflipbook false false)
  (Audio|Components|Audio|Stop _frontflipbook)
  (Rendering|SetVisibility _frontflipbook false false))

(fn SetSpikesUp
  (bind _backflipbook (Variables|Default|GetBackFlipbook))
  (bind _frontflipbook (Variables|Default|GetFrontFlipbook))
  (Utilities|FlowControl|Sequence
    (:then_0
      (if (!= (Class|PaperFlipbookComponent|GetPlaybackPositioninFrames (Variables|Default|GetBackFlipbook)) (Variables|Default|GetActivationFlipbookLengthUp))
        (Class|PaperFlipbookComponent|SetPlaybackPositioninFrames _backflipbook (Variables|Default|GetActivationFlipbookLengthUp) false)
        (Audio|Components|Audio|Stop _backflipbook))
      (if (not (Rendering|IsVisible _backflipbook))
        (Rendering|SetVisibility _backflipbook true false)))
    (:then_1
      (if (!= (Class|PaperFlipbookComponent|GetPlaybackPositioninFrames (Variables|Default|GetFrontFlipbook)) (Variables|Default|GetActivationFlipbookLengthUp))
        (Class|PaperFlipbookComponent|SetPlaybackPositioninFrames _frontflipbook (Variables|Default|GetActivationFlipbookLengthDown) false)
        (Audio|Components|Audio|Stop _frontflipbook))
      (if (not (Rendering|IsVisible _frontflipbook))
        (Rendering|SetVisibility _frontflipbook true false)))
    (:then_2
      (return))))

(fn ShowSpikes
  (Rendering|SetVisibility (Variables|Default|GetBackFlipbook) true false)
  (Rendering|SetVisibility (Variables|Default|GetFrontFlipbook) true false))