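; Potion pickup prop whose Picked event hides its sprite, plays visual and audio feedback, then removes the actor.
; A delay-based flash macro waits for the drinking animation to advance, then blinks FlashPlane twice as a red screen flash.
; When the flashes end it plays the pickup sound, and the audio-finished callback destroys the potion.
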(event Custom|PotionPickedAudioFinished
  (Actor|DestroyActor))

(event EventBeginPlay)

(event EventActorBeginOverlap
  (params (OtherActor :type Actor%20Object%20Reference)))

(event EventTick
  (params (DeltaSeconds :type Float%20%28single-precision%29)))

(event EventPicked
  (params (Prince :type Prince%20Character%20Object%20Reference))
  (Rendering|SetVisibility (Variables|Default|GetCenterSprite) false true)
  (Development|PrintString "Potion picked")
  (EventDispatchers|BindEventtoOnAudioFinished (Variables|Default|GetAudio) (delegate Custom|PotionPickedAudioFinished))
  (Utilities|PotionPickedFlash
    (:End
      (CallFunction|PlaySound (Variables|Default|GetPotionPickedSound) (Variables|Default|GetAudio)))))

(fn ConstructionScript
  (|CallParentFunction))