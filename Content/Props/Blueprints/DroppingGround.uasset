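; DroppingGround is the falling floor piece, linked to a TremblingGround, that drops and crashes onto what lies below.
; Activate reveals it, line-traces for an adjacent Ground, PillarsBrick or WallBrick to show its border, then enables physics and gravity on the sprite.
; The first valid collision overlap hides it, tells the hit actor to show garbage and plays a crash sound.
; It destroys itself shortly after the sound finishes.
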(event OnComponentBeginOverlap(CollisionBox)
  (params (OtherActor :type Actor%20Object%20Reference) (OtherComp :type Primitive%20Component%20Object%20Reference) (OtherBodyIndex :type Integer) (bFromSweep :type Boolean) (SweepResult :type Hit%20Result%20Structure%20%28by%20ref%29))
  (bind _audio (Variables|Default|GetAudio))
  ;[1 1 1] Crash against floor
  (Utilities|Casting|CastToTremblingGround OtherActor
    (:CastFailed
      (Utilities|Casting|CastToCameraChangerGate OtherActor
        (:CastFailed
          (if (and (!= OtherActor (Variables|Default|GetAdjacentGround)) (not (Variables|Default|GetCrashed)))
            (Utilities|FlowControl|Sequence
              (:then_0
                (Rendering|SetActorHiddenInGame true))
              (:then_1
                (Class|GroundInterface|ShowGarbage(Message) OtherActor))
              (:then_2
                ;;[1 1 1] Crashing sound
                (EventDispatchers|BindEventtoOnAudioFinished _audio (delegate Custom|OnGroundCrashingSoundFinished))
                (CallFunction|PlaySound "/Game/Sound/Effects/ground_crashing.ground_crashing" _audio))
              (:then_3
                (Variables|Default|SetCrashed true)))))))))

(event Custom|OnGroundCrashingSoundFinished
  ;[1 1 1] Crash against floor
  ;;[1 1 1] Crashing sound
  (EventDispatchers|UnbindEventfromOnAudioFinished (Variables|Default|GetAudio) (delegate Custom|OnGroundCrashingSoundFinished))
  ;;;[1 1 1] It should not be needed but if I don't use this Audio component gives an error because it says it tries to play while pending to be killed.
  (Utilities|FlowControl|Delay 0.4)
  (Actor|DestroyActor))

(fn ConstructionScript)

(fn Activate
  (bind _centersprite (Variables|Default|GetCenterSprite))
  (Utilities|FlowControl|Sequence
    (:then_0
      ;[1 1 1] Show falling floor.
      (Rendering|SetActorHiddenInGame false))
    (:then_1
      ;[1 1 1] If floor fall without updating adjacent ground it could remain with no border.
      (bind (_adjacentground _borderactordetected) (CallFunction|AdjacentGround?))
      (if _adjacentground
        (bind _output_get (Variables|Default|SetAdjacentGround _borderactordetected))
        (Class|BorderInterface|ShowBorder(Message) _output_get true)))
    (:then_2
      ;[1 1 1] Let it fall.
      (Physics|SetSimulatePhysics _centersprite true)
      (Physics|SetEnableGravity _centersprite true))
    (:then_3
      (Collision|SetCollisionEnabled (Variables|Default|GetCenterSprite) "QueryOnly"))))

(fn SetTremblingFather
  (params (TremblingFather :type Trembling%20Ground%20Object%20Reference))
  (Variables|Default|SetTremblingFather TremblingFather))

(fn AdjacentGround?
  (bind _asprince_character (Utilities|Casting|CastToPrinceCharacter (Game|GetPlayerCharacter 0)))
  (bind (_outhit _returnvalue) (Collision|LineTraceByChannel (Transformation|GetWorldLocation (Variables|Default|GetAdjacentGroundDetectorStart)) (Transformation|GetWorldLocation (Variables|Default|GetAdjacentGroundDetectorEnd)) "TraceTypeQuery1" false (Utilities|Array|MakeArray _asprince_character) "Persistent"))
  (if _returnvalue
    (Utilities|Casting|CastToGround (.HitActor (Collision|BreakHitResult _outhit))
      (:then
        (Variables|Default|SetAdjacencyDetected true :!label _label))
      (:CastFailed
        (Utilities|Casting|CastToPillarsBrick (.HitActor (Collision|BreakHitResult _outhit))
          (:then
            (goto _label))
          (:CastFailed
            (Utilities|Casting|CastToWallBrick (.HitActor (Collision|BreakHitResult _outhit))
              (:then
                (goto _label))
              (:CastFailed
                (Variables|Default|SetAdjacencyDetected false :!label _label_2)))))))
    (else
      (goto _label_2)))
  (return (Variables|Default|GetAdjacencyDetected) (.HitActor (Collision|BreakHitResult _outhit))))