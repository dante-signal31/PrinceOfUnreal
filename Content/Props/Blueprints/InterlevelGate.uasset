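; Interlevel exit gate that lets the Prince leave for the next level.
; A state machine and timelines raise or lower the panel on Tick, with slow and fast closing.
; RangeBox overlaps while opening or open register the gate with the character, enabling EnterGate.
; The entering flipbook, shifted in depth mid-play, chains into win music and an optional video timed by accumulated delta seconds, then loads NextLevel.
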(event OnComponentBeginOverlap(RangeBox)
  (params (OtherActor :type Actor%20Object%20Reference) (OtherComp :type Primitive%20Component%20Object%20Reference) (OtherBodyIndex :type Integer) (bFromSweep :type Boolean) (SweepResult :type Hit%20Result%20Structure%20%28by%20ref%29))
  ;[1 1 1] Can character change level?
  (bind _asprince_character (Utilities|Casting|CastToPrinceCharacter OtherActor))
  (switch Utilities|FlowControl|Switch|SwitchonGateStates (Variables|Default|GetState)
    (:NewEnumerator1
      _)
    (:NewEnumerator3
      _))
  (Variables|Default|SetChangingLevelAllowed true)
  (Default|SetInterlevelGateAvailable _asprince_character self)
  (Development|PrintString "Changing level allowed"))

(event OnComponentEndOverlap(RangeBox)
  (params (OtherActor :type Actor%20Object%20Reference) (OtherComp :type Primitive%20Component%20Object%20Reference) (OtherBodyIndex :type Integer))
  ;[1 1 1] Can character change level?
  (bind _asprince_character (Utilities|Casting|CastToPrinceCharacter OtherActor))
  (Variables|Default|SetChangingLevelAllowed false)
  (Default|RemoveInterlevelGateAvailable _asprince_character)
  (Development|PrintString "Changing level not allowed"))

(event Custom|PlayEndLevelMusic
  (bind _winmusic (Variables|Default|GetWinMusic))
  ;[1 1 1] BeginPlay setup
  ;;[1 1 1] Entering final gate sequence setup
  ;;;[0.3414 0.3421 1] Music
  (CallFunction|HideAnimation)
  (EventDispatchers|BindEventtoOnAudioFinished (Variables|Default|GetAudio) (delegate Custom|ChangeLevel))
  (if (!= 0 _winmusic)
    (CallFunction|PlaySound _winmusic (Variables|Default|GetAudio))
    (else
      (CallFunction|ChangeLevel)))
  (EventDispatchers|UnbindEventfromOnFinishedPlaying (Variables|Default|GetEnteringGateAnimation) (delegate Custom|PlayEndLevelMusic)))

(event Custom|ChangeLevel
  (bind _endlevelvideoplayer (Variables|Default|GetEndLevelVideoPlayer))
  (bind _endlevelvideoimagematerial (Variables|Default|GetEndLevelVideoImageMaterial))
  ;[1 1 1] BeginPlay setup
  ;;[1 1 1] Entering final gate sequence setup
  ;;;[0.3414 0.3421 1] Interlevel video
  (EventDispatchers|UnbindEventfromOnAudioFinished (Variables|Default|GetAudio) (delegate Custom|ChangeLevel))
  (if (and (!= _endlevelvideoplayer 0) (!= _endlevelvideoimagematerial 0))
    (CallFunction|SetHudVisibility false)
    (bind (_isplaying_ _videolength) (CallFunction|ShowVideo 0 (Variables|Default|GetAudio) (Variables|Default|GetEndLevelVideoMusic) _endlevelvideoplayer _endlevelvideoimagematerial))
    (Variables|Default|SetplayingVideo _isplaying_)
    (Variables|Default|SetVideoLength _videolength)
    (else
      (Variables|Default|SetChangeLevelNow true))))

(event EventOpenGate
  (bind _audio (Variables|Default|GetAudio))
  ;[1 1 1] Open
  (switch Utilities|FlowControl|Switch|SwitchonGateStates (Variables|Default|GetState)
    (:NewEnumerator0
      (Variables|Default|SetState "NewEnumerator1" :!label _label)
      (CallFunction|PlaySound (Variables|Default|GetPanelSound) _audio)
      ;[1 1 1] Change panel elevation
      (bind _panelelevation (Timeline|OpenInterlevelGate PlayFromStart)
        (:Update
          (Variables|Default|SetElevationProportion _panelelevation))))
    (:NewEnumerator1
      (goto _label))
    (:NewEnumerator2
      (Variables|Default|SetState "NewEnumerator1" :!label _label_2)
      (CallFunction|PlaySound (Variables|Default|GetPanelSound) _audio)
      (Timeline|OpenInterlevelGate Play))
    (:NewEnumerator4
      (goto _label_2))))

(event EventTick
  (params (DeltaSeconds :type Float%20%28single-precision%29))
  (bind _audio (Variables|Default|GetAudio))
  (bind _elevationproportion (Variables|Default|GetElevationProportion))
  ;[1 1 1] Tick
  (switch Utilities|FlowControl|Switch|SwitchonGateStates (Variables|Default|GetState)
    (:NewEnumerator1
      ;;[0.3414 0.3421 1] Elevate panel
      (CallFunction|MovePanel _elevationproportion)
      (if (>= _elevationproportion 1.0)
        (Variables|Default|SetState "NewEnumerator3")
        (CallFunction|StopSound (Variables|Default|GetAudio))))
    (:NewEnumerator3
      (Utilities|FlowControl|Sequence
        (:then_0
          ;;[0.3414 0.3421 1] Load next level
          (if (Variables|Default|GetChangeLevelNow)
            (CallFunction|SetHudVisibility true)
            (Game|OpenLevel(byName) (Variables|Default|GetNextLevel))))
        (:then_1
          (CallFunction|UpdateAnimationDeep))
        (:then_2
          ;;[0.3414 0.3421 1] Check intelevel video ended
          (if (Variables|Default|GetplayingVideo)
            (bind _returnvalue (CallFunction|EndLevelVideoEnded? DeltaSeconds))
            (if _returnvalue
              (Utilities|FlowControl|Sequence
                (:then_0
                  (Variables|Default|SetCurrentVideoTime (Math|Timespan|FromSeconds 0.0))
                  (Variables|Default|SetplayingVideo false))
                (:then_1
                  (Variables|Default|SetChangeLevelNow true))))))))
    (:NewEnumerator2
      ;;[0.3414 0.3421 1] Descend panel
      (CallFunction|MovePanel _elevationproportion :!label _label)
      (if (<= _elevationproportion 0.0)
        (switch Utilities|FlowControl|Switch|SwitchonGateStates (Variables|Default|GetState)
          (:NewEnumerator2
            (CallFunction|StopSound _audio))
          (:NewEnumerator4
            (CallFunction|PlaySound (Variables|Default|GetPanelSoundClosingFast) _audio)))
        (Variables|Default|SetState "NewEnumerator0")))
    (:NewEnumerator4
      (goto _label))))

(event EventCloseGateSlow
  (bind _audio (Variables|Default|GetAudio))
  ;[1 1 1] Close slow
  (switch Utilities|FlowControl|Switch|SwitchonGateStates (Variables|Default|GetState)
    (:NewEnumerator1
      (Variables|Default|SetState "NewEnumerator2")
      (CallFunction|PlaySound (Variables|Default|GetPanelSound) _audio)
      ;[1 1 1] Change panel elevation
      (bind _panelelevation (Timeline|OpenInterlevelGate Reverse)
        (:Update
          (Variables|Default|SetElevationProportion _panelelevation))))
    (:NewEnumerator3
      (Variables|Default|SetState "NewEnumerator2" :!label _label)
      (CallFunction|PlaySound (Variables|Default|GetPanelSound) _audio)
      (Timeline|OpenInterlevelGate ReverseFromEnd))
    (:NewEnumerator2
      (goto _label))
    (:NewEnumerator4
      (goto _label))))

(event EventCloseGateFast
  ;[1 1 1] Close fast
  (switch Utilities|FlowControl|Switch|SwitchonGateStates (Variables|Default|GetState)
    (:NewEnumerator1
      (bind _panelelevation (Timeline|CloseFastInterlevelGate Play)
        (:Update
          (Variables|Default|SetElevationProportion _panelelevation)
          (Variables|Default|SetState "NewEnumerator4"))))
    (:NewEnumerator3
      (Timeline|CloseFastInterlevelGate PlayFromStart))))

(event EventBeginPlay
  ;[1 1 1] BeginPlay setup
  (Utilities|FlowControl|Sequence
    (:then_0
      (CallFunction|InitMovement))
    (:then_1
      ;;[1 1 1] Entering final gate sequence setup
      (EventDispatchers|BindEventtoOnFinishedPlaying (Variables|Default|GetEnteringGateAnimation) (delegate Custom|PlayEndLevelMusic)))))

(fn ConstructionScript
  (Utilities|FlowControl|Sequence
    (:then_0
      ;[1 1 1] Prince entering gate animation setup.
      (CallFunction|HideAnimation)
      (CallFunction|DisableAnimationLooping))
    (:then_1
      (CallFunction|GetAnimationLocation))
    (:then_2
      ;[1 1 1] Closing panel setup
      (CallFunction|GetClosedElevation))
    (:then_3
      (CallFunction|SetInitialPanelSetup))))

(fn MovePanel
  (params (Elevation :type Float%20%28single-precision%29))
  (bind _panelsprite (Variables|Default|GetPanelSprite))
  (bind _relativelocation (Variables|/Script/Engine.SceneComponent|GetRelativeLocation _panelsprite))
  (Transformation|SetRelativeLocation _panelsprite (Math|Vector|MakeVector (.x _relativelocation) (.y _relativelocation) (+ (Variables|Default|GetClosedElevation) (* Elevation (Variables|Default|GetMaximumElevation)))) false false))

(fn GetClosedElevation
  (bind _panelsprite (Variables|Default|GetPanelSprite))
  (bind _relativelocation (Variables|/Script/Engine.SceneComponent|GetRelativeLocation _panelsprite))
  (bind _output_get (Variables|Default|SetClosedElevation (.z _relativelocation)))
  (Variables|Default|SetPanelDefaultRelativeLocation (Math|Vector|MakeVector (.x _relativelocation) (.y _relativelocation) _output_get))
  (return))

(fn StopSound
  (Audio|Components|Audio|Stop (Variables|Default|GetAudio)))

(fn EnterGate
  (if (Variables|Default|GetChangingLevelAllowed)
    (Utilities|FlowControl|Sequence
      (:then_0
        (CallFunction|ShowAnimation)))))

(fn SetInitialPanelSetup
  (switch Utilities|FlowControl|Switch|SwitchonGateStates (Variables|Default|GetInitialState)
    (:NewEnumerator0
      _)
    (:NewEnumerator1
      _)
    (:NewEnumerator3
      (CallFunction|SetGateasOpen :!label _label))
    (:NewEnumerator2
      (goto _label))
    (:NewEnumerator4
      (goto _label)))
  (Variables|Default|SetState (Variables|Default|GetInitialState)))

(fn SetGateasOpen
  (bind _paneldefaultrelativelocation (Variables|Default|GetPanelDefaultRelativeLocation))
  (Transformation|SetRelativeLocation (Variables|Default|GetPanelSprite) (Math|Vector|MakeVector (.x _paneldefaultrelativelocation) (.y _paneldefaultrelativelocation) (+ (.z _paneldefaultrelativelocation) (Variables|Default|GetMaximumElevation))) false true)
  (return))

(fn InitMovement
  (switch Utilities|FlowControl|Switch|SwitchonGateStates (Variables|Default|GetInitialState)
    (:NewEnumerator0
      _)
    (:NewEnumerator1
      (CallFunction|OpenGate))
    (:NewEnumerator3
      _)
    (:NewEnumerator2
      (CallFunction|CloseGateSlow))
    (:NewEnumerator4
      (CallFunction|CloseGateFast)))
  (return))

(fn GetAnimationLocation
  (Variables|Default|SetEnteringGateAnimationInitialLocation (Variables|/Script/Engine.SceneComponent|GetRelativeLocation (Variables|Default|GetEnteringGateAnimation)))
  (return))

(fn UpdateAnimationDeep
  (bind _enteringgateanimation (Variables|Default|GetEnteringGateAnimation))
  (bind _enteringgateanimationinitiallocation (Variables|Default|GetEnteringGateAnimationInitialLocation))
  (bind _returnvalue (Class|PaperFlipbookComponent|GetPlaybackPositioninFrames _enteringgateanimation))
  (if (Variables|Default|GetEnterGateAnimationEnabled)
    (if (== _returnvalue 0)
      (Transformation|SetRelativeLocation _enteringgateanimation (Math|Vector|MakeVector (.x _enteringgateanimationinitiallocation) (.y _enteringgateanimationinitiallocation) (.z _enteringgateanimationinitiallocation)) false true)
      (elif (== _returnvalue 6)
        (Transformation|SetRelativeLocation _enteringgateanimation (Math|Vector|MakeVector (.x _enteringgateanimationinitiallocation) (Variables|Default|GetAnimationEndDeep) (.z _enteringgateanimationinitiallocation)) false true))))
  (return))

(fn HideAnimation
  (bind _enteringgateanimation (Variables|Default|GetEnteringGateAnimation))
  (Audio|Components|Audio|Stop _enteringgateanimation)
  (Rendering|SetVisibility _enteringgateanimation false false)
  (return))

(fn ShowAnimation
  (bind _enteringgateanimation (Variables|Default|GetEnteringGateAnimation))
  (Rendering|SetVisibility _enteringgateanimation true false)
  (Components|Timeline|PlayfromStart _enteringgateanimation)
  (return))

(fn DisableAnimationLooping
  (Components|Timeline|SetLooping (Variables|Default|GetEnteringGateAnimation) false)
  (return))

(fn UpdateCurrentVideoTime
  (params (Seconds :type Float%20%28single-precision%29))
  (bind _output_get (Variables|Default|SetCurrentVideoTime (+ (Variables|Default|GetCurrentVideoTime) (Math|Timespan|FromSeconds Seconds))))
  (return _output_get))

(fn EndLevelVideoEnded?
  (params (Seconds :type Float%20%28single-precision%29))
  (bind _updatedcurrentvideotime (CallFunction|UpdateCurrentVideoTime Seconds))
  (return (>= _updatedcurrentvideotime (Variables|Default|GetVideoLength))))