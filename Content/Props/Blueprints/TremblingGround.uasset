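; Loose floor prop that trembles and then falls when the PrinceCharacter enters its FallingBox.
; When the animation ends, it spawns and activates a DroppingGround, removes itself from the current level camera and destroys itself.
; It can also subscribe to the Prince's landing dispatcher, trembling without falling if he lands within ProximityBox.
; Both behaviors share one animation-and-sound routine, binding different OnFinishedPlaying handlers to decide the outcome.
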(event OnComponentBeginOverlap(FallingBox)
  (params (OtherActor :type Actor%20Object%20Reference) (OtherComp :type Primitive%20Component%20Object%20Reference) (OtherBodyIndex :type Integer) (bFromSweep :type Boolean) (SweepResult :type Hit%20Result%20Structure%20%28by%20ref%29))
  (Utilities|Casting|CastToPrinceCharacter OtherActor)
  ;[1 1 1] Tremble, dissapear and launch falling ground.
  (Utilities|FlowControl|Sequence
    (:then_0
      (EventDispatchers|BindEventtoOnFinishedPlaying (Variables|Default|GetTremblingAnimation) (delegate Custom|InitDropping))
      (CallFunction|PlayTremblingAnimation))))

(event Custom|bindToLandingEventDispatcher
  (params (Prince :type Prince%20Character%20Object%20Reference))
  ;[1 1 1] Subscribe to receive vibrations.
  (EventDispatchers|BindEventtoLandingEventDispatcher Prince (delegate Custom|OnVibrationReceived)))

(event Custom|unbindToLandingEventDispatcher
  (params (Prince :type Prince%20Character%20Object%20Reference))
  ;[1 1 1] End receiving vibration notifications.
  (EventDispatchers|UnbindEventfromLandingEventDispatcher Prince (delegate Custom|OnVibrationReceived)))

(event Custom|AnimationEnded
  (bind _tremblinganimation (Variables|Default|GetTremblingAnimation))
  ;[1 1 1] Subscribe to receive vibrations.
  (Rendering|SetVisibility _tremblinganimation false false)
  (EventDispatchers|UnbindEventfromOnFinishedPlaying _tremblinganimation (delegate Custom|AnimationEnded)))

(event Custom|InitDropping
  ;[1 1 1] Tremble, dissapear and launch falling ground.
  (Rendering|SetVisibility (Variables|Default|GetTremblingAnimation) false false)
  (Utilities|FlowControl|Delay 0.4)
  (bind _returnvalue (Game|SpawnActorfromClass "/Game/Props/Blueprints/DroppingGround.DroppingGround_C" (Math|Transform|MakeTransform (.Location (Math|Transform|BreakTransform (Transformation|GetWorldTransform (Variables|Default|GetCenterSprite))))) "AdjustIfPossibleButAlwaysSpawn" 0 0))
  (Default|SetTremblingFather _returnvalue self)
  (Default|Activate _returnvalue)
  (bind _asprince_game_state (Utilities|Casting|CastToPrinceGameState (Game|GetGameState)))
  (bind _currentcamera (Default|GetCurrentLevelCamera _asprince_game_state))
  (Default|RemoveTremblingGround _currentcamera self)
  (Utilities|FlowControl|Delay 0.1)
  (Actor|DestroyActor))

(event Custom|OnVibrationReceived
  ;[1 1 1] Subscribe to receive vibrations.
  (if (CallFunction|IsPrinceNearEnough)
    (EventDispatchers|BindEventtoOnFinishedPlaying (Variables|Default|GetTremblingAnimation) (delegate Custom|AnimationEnded))
    (CallFunction|PlayTremblingAnimation)))

(fn ConstructionScript
  (|CallParentFunction)
  (Utilities|FlowControl|Sequence
    (:then_0
      (Rendering|SetVisibility (Variables|Default|GetTremblingAnimation) false false))))

(fn PlayTremblingAnimation
  (bind _tremblinganimation (Variables|Default|GetTremblingAnimation))
  (Rendering|SetVisibility (Variables|Default|GetOcluder) false false)
  (Components|Timeline|SetLooping _tremblinganimation false)
  (Rendering|SetVisibility _tremblinganimation true false)
  (Utilities|FlowControl|Sequence
    (:then_0
      (Components|Timeline|PlayfromStart _tremblinganimation))
    (:then_1
      (CallFunction|PlaySound (Variables|Default|GetTremblingSound) (Variables|Default|GetAudio)))))

(fn ActivateFalling
  (bind _asprince_game_state (Utilities|Casting|CastToPrinceGameState (Game|GetGameState)))
  (bind _currentcamera (Default|GetCurrentLevelCamera _asprince_game_state))
  (Default|RemoveTremblingGround _currentcamera self)
  (Actor|DestroyActor))

(fn IsPrinceNearEnough
  (bind _actorsfound (CallFunction|GetInstancesinArea (Variables|Default|GetProximityBox) "/Game/Characters/PrinceCharacter.PrinceCharacter_C"))
  (return (> (Utilities|Array|Length _actorsfound) 0)))