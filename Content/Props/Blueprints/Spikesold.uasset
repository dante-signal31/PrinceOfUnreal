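; Spike trap prop for a Prince of Persia-style 2D game that kills the prince if he runs, lands or falls onto it.
; A proximity volume raises and retracts two spike flipbooks by playing them forward or reversed, with finish events updating the trap state.
; A killing volume checks the prince's movement state, applies damage, tints the camera red, swaps him for a corpse sprite, then reloads the level after the death music.
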(event OnComponentBeginOverlap(ProximityVolume)
  (params (OtherActor :type Actor%20Object%20Reference) (OtherComp :type Primitive%20Component%20Object%20Reference) (OtherBodyIndex :type Integer) (bFromSweep :type Boolean) (SweepResult :type Hit%20Result%20Structure%20%28by%20ref%29))
  ;[1 1 1] Entering spikes range
  (Utilities|Casting|CastToPrinceCharacter OtherActor)
  (Variables|Default|SetCurrentState "NewEnumerator1")
  (CallFunction|ActivatingSpikes))

(event OnComponentEndOverlap(ProximityVolume)
  (params (OtherActor :type Actor%20Object%20Reference) (OtherComp :type Primitive%20Component%20Object%20Reference) (OtherBodyIndex :type Integer))
  ;[1 1 1] Leaving spikes range
  (Utilities|Casting|CastToPrinceCharacter OtherActor)
  (Variables|Default|SetCurrentState "NewEnumerator4")
  (CallFunction|DeactivatingSpikes))

(event OnComponentBeginOverlap(KillingVolume)
  (params (OtherActor :type Actor%20Object%20Reference) (OtherComp :type Primitive%20Component%20Object%20Reference) (OtherBodyIndex :type Integer) (bFromSweep :type Boolean) (SweepResult :type Hit%20Result%20Structure%20%28by%20ref%29))
  (bind _audio (Variables|Default|GetAudio))
  ;[1 1 1] Into the killing zone
  (bind _asprince_character (Utilities|Casting|CastToPrinceCharacter OtherActor))
  (switch Utilities|FlowControl|Switch|SwitchonPrinceStates (Default|GetState _asprince_character)
    (:NewEnumerator1
      _)
    (:NewEnumerator2
      _)
    (:NewEnumerator3
      _)
    (:NewEnumerator22
      _)
    (:NewEnumerator16
      (CallFunction|PlaySound (Variables|Default|GetChaftSound) (Variables|Default|GetAudio) :!label _label))
    (:NewEnumerator6
      (goto _label)))
  (Utilities|FlowControl|Sequence
    (:then_0
      ;;[0.3414 0.3421 1] Apply damage to prince character
      (Game|Damage|ApplyDamage _asprince_character 1.0 0 self))
    (:then_1
      ;;[0.3414 0.3421 1] Disable actor
      (Actor|Tick|SetActorTickEnabled _asprince_character))
    (:then_2
      ;;[0.3414 0.3421 1] Red screen flash
      (bind _asprince_game_state (Utilities|Casting|CastToPrinceGameState (Game|GetGameState)))
      (bind _currentcamera (Default|GetCurrentLevelCamera _asprince_game_state))
      (Default|TintRed _currentcamera)
      (Utilities|FlowControl|Delay (Variables|Default|GetRedTintShowtime))
      (Default|RemoveTint _currentcamera))
    (:then_3
      ;;[0.3414 0.3421 1] Show death sprites
      (CallFunction|ShowDamageSignal)
      (Rendering|SetActorHiddenInGame _asprince_character true)
      (CallFunction|RotateCorpse _asprince_character)
      (CallFunction|ShowCorpse)
      (Utilities|FlowControl|Delay (Variables|Default|GetDamageSignalShowtime))
      (CallFunction|HideDamageSignal)
      (Utilities|FlowControl|Delay (Variables|Default|GetDeathMusicWaitingTime))
      ;;[0.3414 0.3421 1] Play death music
      (CallFunction|PlaySound (Variables|Default|GetDeathMusic) _audio)
      ;;[0.3414 0.3421 1] Restart level
      (EventDispatchers|BindEventtoOnAudioFinished _audio (delegate Custom|RestartLevel)))))

(event Custom|SpikesDeactivated
  ;[1 1 1] Spikes deactivation
  (CallFunction|HideSpikes)
  (Variables|Default|SetCurrentState "NewEnumerator0")
  (EventDispatchers|UnbindEventfromOnFinishedPlaying (Variables|Default|GetUpSpikes) (delegate Custom|SpikesDeactivated)))

(event Custom|SpikesActivated
  ;[1 1 1] Spikes activation
  (Variables|Default|SetCurrentState "NewEnumerator2")
  (EventDispatchers|UnbindEventfromOnFinishedPlaying (Variables|Default|GetUpSpikes) (delegate Custom|SpikesActivated)))

(event Custom|ActivatingSpikes
  (bind _upspikes (Variables|Default|GetUpSpikes))
  (bind _downspikes (Variables|Default|GetDownSpikes))
  ;[1 1 1] Spikes activation
  (CallFunction|PlaySound (Variables|Default|GetSpikesActivationSound) (Variables|Default|GetAudio))
  (EventDispatchers|BindEventtoOnFinishedPlaying _upspikes (delegate Custom|SpikesActivated))
  (Rendering|SetVisibility _upspikes true false)
  (Components|Timeline|PlayfromStart _upspikes)
  (Rendering|SetVisibility _downspikes true false)
  (Components|Timeline|PlayfromStart _downspikes))

(event Custom|DeactivatingSpikes
  (bind _upspikes (Variables|Default|GetUpSpikes))
  ;[1 1 1] Spikes deactivation
  (EventDispatchers|BindEventtoOnFinishedPlaying _upspikes (delegate Custom|SpikesDeactivated))
  (Components|Timeline|ReversefromEnd _upspikes)
  (Components|Timeline|ReversefromEnd (Variables|Default|GetDownSpikes)))

(event Custom|RestartLevel
  ;[1 1 1] Into the killing zone
  ;;[0.3414 0.3421 1] Restart level
  (EventDispatchers|UnbindEventfromOnAudioFinished (Variables|Default|GetAudio) (delegate Custom|RestartLevel))
  (CallFunction|ReloadLevel))

(event EventBeginPlay)

(event EventActorBeginOverlap
  (params (OtherActor :type Actor%20Object%20Reference)))

(event EventTick
  (params (DeltaSeconds :type Float%20%28single-precision%29)))

(fn ConstructionScript
  (Utilities|FlowControl|Sequence
    (:then_0
      (Variables|Default|SetCurrentState (Variables|Default|GetInitialState))
      (Variables|Default|SetActivationFlipbookLengthUp (Class|PaperFlipbookComponent|GetFlipbookLengthinFrames (Variables|Default|GetUpSpikes)))
      (Variables|Default|SetActivationFlipbookLengthDown (Class|PaperFlipbookComponent|GetFlipbookLengthinFrames (Variables|Default|GetDownSpikes))))
    (:then_1
      (CallFunction|DeactivateSpikesAnimationLooping))
    (:then_2
      (switch Utilities|FlowControl|Switch|SwitchonTrapStates (Variables|Default|GetCurrentState)
        (:NewEnumerator0
          (CallFunction|HideSpikes :!label _label)
          (CallFunction|HideCorpse :!label _label_2)
          (CallFunction|HideDamageSignal))
        (:NewEnumerator1
          (goto _label))
        (:NewEnumerator2
          (CallFunction|SetSpikesUp :!label _label_3)
          (goto _label_2))
        (:NewEnumerator3
          (CallFunction|SetSpikesUp)
          (CallFunction|ShowCorpse))
        (:NewEnumerator4
          (goto _label_3))))
    (:then_3
      (CallFunction|SetInitialFrames))))

(fn HideSpikes
  (bind _upspikes (Variables|Default|GetUpSpikes))
  (bind _downspikes (Variables|Default|GetDownSpikes))
  (Audio|Components|Audio|Stop _upspikes)
  (Rendering|SetVisibility _upspikes false false)
  (Audio|Components|Audio|Stop _downspikes)
  (Rendering|SetVisibility _downspikes false false)
  (return))

(fn SetInitialFrames
  (bind _ground (Variables|Default|GetGround))
  (if (Variables|Default|GetHasBorder)
    (Rendering|Components|Sprite|SetSprite _ground (Variables|Default|GetGroundSprite))
    (else
      (Rendering|Components|Sprite|SetSprite _ground (Variables|Default|GetGroundNoBorderSprite))))
  (return))

(fn SetSpikesUp
  (bind _upspikes (Variables|Default|GetUpSpikes))
  (bind _downspikes (Variables|Default|GetDownSpikes))
  (Utilities|FlowControl|Sequence
    (:then_0
      (if (!= (Class|PaperFlipbookComponent|GetPlaybackPositioninFrames (Variables|Default|GetUpSpikes)) (Variables|Default|GetActivationFlipbookLengthUp))
        (Class|PaperFlipbookComponent|SetPlaybackPositioninFrames _upspikes (Variables|Default|GetActivationFlipbookLengthUp) false)
        (Audio|Components|Audio|Stop _upspikes))
      (if (not (Rendering|IsVisible (Variables|Default|GetUpSpikes)))
        (Rendering|SetVisibility _upspikes true false)))
    (:then_1
      (if (!= (Class|PaperFlipbookComponent|GetPlaybackPositioninFrames (Variables|Default|GetDownSpikes)) (Variables|Default|GetActivationFlipbookLengthUp))
        (Class|PaperFlipbookComponent|SetPlaybackPositioninFrames _downspikes (Variables|Default|GetActivationFlipbookLengthDown) false)
        (Audio|Components|Audio|Stop _downspikes))
      (if (not (Rendering|IsVisible (Variables|Default|GetDownSpikes)))
        (Rendering|SetVisibility _downspikes true false)))
    (:then_2
      (return))))

(fn HideCorpse
  (Rendering|SetVisibility (Variables|Default|GetCorpse) false false)
  (return))

(fn ShowCorpse
  (Rendering|SetVisibility (Variables|Default|GetCorpse) true false)
  (return))

(fn DeactivateSpikesAnimationLooping
  (Components|Timeline|SetLooping (Variables|Default|GetUpSpikes) false)
  (Components|Timeline|SetLooping (Variables|Default|GetDownSpikes) false)
  (return))

(fn ActivateSpikes
  (CallFunction|PlaySound (Variables|Default|GetSpikesActivationSound) (Variables|Default|GetAudio))
  (Components|Timeline|PlayfromStart (Variables|Default|GetUpSpikes))
  (Components|Timeline|PlayfromStart (Variables|Default|GetDownSpikes))
  (return))

(fn HideDamageSignal
  (Rendering|SetVisibility (Variables|Default|GetDamageSignal) false false)
  (return))

(fn ShowDamageSignal
  (Rendering|SetVisibility (Variables|Default|GetDamageSignal) true false)
  (return))

(fn RotateCorpse
  (params (PrinceCharacter :type Prince%20Character%20Object%20Reference))
  (if (Default|IsRightwards PrinceCharacter)
    _
    (else
      (Transformation|SetWorldRotation (Variables|Default|GetCorpse) "0,180.000000, 0" false false)))
  (return))

(fn ReloadLevel
  (bind _returnvalue (Game|GetCurrentLevelName true))
  (Game|OpenLevel(byName) (Utilities|String|StringToName _returnvalue))
  (return))