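; Paper2D spike trap prop that rises when the PrinceCharacter enters its proximity volume and retracts when it leaves.
; Overlaps set the state and play the upper and lower flipbooks forward with sound or in reverse, with finished-playing callbacks settling it to Active or Inactive.
; The construction script previews InitialState, setting spike and corpse visibility and the bordered or borderless ground sprite.
; Killing only affects that initial setup, and Tick's state switch is empty.
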(event OnComponentBeginOverlap(ProximityVolume)
  (params (OtherActor :type Actor%20Object%20Reference) (OtherComp :type Primitive%20Component%20Object%20Reference) (OtherBodyIndex :type Integer) (bFromSweep :type Boolean) (SweepResult :type Hit%20Result%20Structure%20%28by%20ref%29))
  (Utilities|Casting|CastToPrinceCharacter OtherActor)
  (Variables|Default|SetCurrentState "NewEnumerator1")
  (CallFunction|ActivatingSpikes))

(event OnComponentEndOverlap(ProximityVolume)
  (params (OtherActor :type Actor%20Object%20Reference) (OtherComp :type Primitive%20Component%20Object%20Reference) (OtherBodyIndex :type Integer))
  (Utilities|Casting|CastToPrinceCharacter OtherActor)
  (Variables|Default|SetCurrentState "NewEnumerator4")
  (CallFunction|DeactivatingSpikes))

(event Custom|SpikesDeactivated
  ;[1 1 1] Spikes deactivation
  (CallFunction|HideSpikes)
  (Variables|Default|SetCurrentState "NewEnumerator0")
  (EventDispatchers|UnbindEventfromOnFinishedPlaying (Variables|Default|GetUpSpikes) (delegate Custom|SpikesDeactivated)))

(event Custom|SpikesActivated
  ;[1 1 1] Spikes activation
  (Variables|Default|SetCurrentState "NewEnumerator2")
  (EventDispatchers|UnbindEventfromOnFinishedPlaying (Variables|Default|GetUpSpikes) (delegate Custom|SpikesActivated)))

(event Custom|ActivatingSpikes
  (bind _upspikes (Variables|Default|GetUpSpikes))
  (bind _downspikes (Variables|Default|GetDownSpikes))
  ;[1 1 1] Spikes activation
  (CallFunction|PlaySound (Variables|Default|GetSpikesActivationSound) (Variables|Default|GetAudio))
  (EventDispatchers|BindEventtoOnFinishedPlaying _upspikes (delegate Custom|SpikesActivated))
  (Rendering|SetVisibility _upspikes true false)
  (Components|Timeline|PlayfromStart _upspikes)
  (Rendering|SetVisibility _downspikes true false)
  (Components|Timeline|PlayfromStart _downspikes))

(event Custom|DeactivatingSpikes
  (bind _upspikes (Variables|Default|GetUpSpikes))
  ;[1 1 1] Spikes deactivation
  (EventDispatchers|BindEventtoOnFinishedPlaying _upspikes (delegate Custom|SpikesDeactivated))
  (Components|Timeline|ReversefromEnd _upspikes)
  (Components|Timeline|ReversefromEnd (Variables|Default|GetDownSpikes)))

(event EventBeginPlay)

(event EventActorBeginOverlap
  (params (OtherActor :type Actor%20Object%20Reference)))

(event EventTick
  (params (DeltaSeconds :type Float%20%28single-precision%29))
  (switch Utilities|FlowControl|Switch|SwitchonSpikesStates (Variables|Default|GetCurrentState)))

(fn ConstructionScript
  (Utilities|FlowControl|Sequence
    (:then_0
      (Variables|Default|SetCurrentState (Variables|Default|GetInitialState))
      (Variables|Default|SetActivationFlipbookLengthUp (Class|PaperFlipbookComponent|GetFlipbookLengthinFrames (Variables|Default|GetUpSpikes)))
      (Variables|Default|SetActivationFlipbookLengthDown (Class|PaperFlipbookComponent|GetFlipbookLengthinFrames (Variables|Default|GetDownSpikes))))
    (:then_1
      (CallFunction|DeactivateSpikesAnimationLooping))
    (:then_2
      (switch Utilities|FlowControl|Switch|SwitchonSpikesStates (Variables|Default|GetCurrentState)
        (:NewEnumerator0
          (CallFunction|HideSpikes :!label _label)
          (CallFunction|HideCorpse :!label _label_2))
        (:NewEnumerator1
          (goto _label))
        (:NewEnumerator2
          (CallFunction|SetSpikesUp :!label _label_3)
          (goto _label_2))
        (:NewEnumerator3
          (CallFunction|SetSpikesUp)
          (CallFunction|ShowCorpse))
        (:NewEnumerator4
          (goto _label_3))))
    (:then_3
      (CallFunction|SetInitialFrames))))

(fn HideSpikes
  (bind _upspikes (Variables|Default|GetUpSpikes))
  (bind _downspikes (Variables|Default|GetDownSpikes))
  (Audio|Components|Audio|Stop _upspikes)
  (Rendering|SetVisibility _upspikes false false)
  (Audio|Components|Audio|Stop _downspikes)
  (Rendering|SetVisibility _downspikes false false)
  (return))

(fn SetInitialFrames
  (bind _ground (Variables|Default|GetGround))
  (if (Variables|Default|GetHasBorder)
    (Rendering|Components|Sprite|SetSprite _ground (Variables|Default|GetGroundSprite))
    (else
      (Rendering|Components|Sprite|SetSprite _ground (Variables|Default|GetGroundNoBorderSprite))))
  (return))

(fn SetSpikesUp
  (bind _upspikes (Variables|Default|GetUpSpikes))
  (bind _downspikes (Variables|Default|GetDownSpikes))
  (Utilities|FlowControl|Sequence
    (:then_0
      (if (!= (Class|PaperFlipbookComponent|GetPlaybackPositioninFrames (Variables|Default|GetUpSpikes)) (Variables|Default|GetActivationFlipbookLengthUp))
        (Class|PaperFlipbookComponent|SetPlaybackPositioninFrames _upspikes (Variables|Default|GetActivationFlipbookLengthUp) false)
        (Audio|Components|Audio|Stop _upspikes))
      (if (not (Rendering|IsVisible (Variables|Default|GetUpSpikes)))
        (Rendering|SetVisibility _upspikes true false)))
    (:then_1
      (if (!= (Class|PaperFlipbookComponent|GetPlaybackPositioninFrames (Variables|Default|GetDownSpikes)) (Variables|Default|GetActivationFlipbookLengthUp))
        (Class|PaperFlipbookComponent|SetPlaybackPositioninFrames _downspikes (Variables|Default|GetActivationFlipbookLengthDown) false)
        (Audio|Components|Audio|Stop _downspikes))
      (if (not (Rendering|IsVisible (Variables|Default|GetDownSpikes)))
        (Rendering|SetVisibility _downspikes true false)))
    (:then_2
      (return))))

(fn HideCorpse
  (Rendering|SetVisibility (Variables|Default|GetCorpse) false false)
  (return))

(fn ShowCorpse
  (Rendering|SetVisibility (Variables|Default|GetCorpse) true false)
  (return))

(fn DeactivateSpikesAnimationLooping
  (Components|Timeline|SetLooping (Variables|Default|GetUpSpikes) false)
  (Components|Timeline|SetLooping (Variables|Default|GetDownSpikes) false)
  (return))

(fn ActivateSpikes
  (CallFunction|PlaySound (Variables|Default|GetSpikesActivationSound) (Variables|Default|GetAudio))
  (Components|Timeline|PlayfromStart (Variables|Default|GetUpSpikes))
  (Components|Timeline|PlayfromStart (Variables|Default|GetDownSpikes))
  (return))