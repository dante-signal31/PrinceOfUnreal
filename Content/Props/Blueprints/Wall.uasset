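; Modular Paper2D wall prop that builds itself in the construction script as a repeating grid of sprite blocks.
; HasGround and HasCutWall choose the sprites for Piece1 and Piece2, then RootSprite's child sprites are recorded with their relative transforms.
; CreateGrid copies the root and those satellites per AmountX and AmountZ, spacing copies by root bounds, with Rightwards and Downwards setting direction.
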(event EventBeginPlay)

(event EventActorBeginOverlap
  (params (OtherActor :type Actor%20Object%20Reference)))

(event EventTick
  (params (DeltaSeconds :type Float%20%28single-precision%29)))

(fn ConstructionScript
  (bind _rootsprite (Variables|Default|GetRootSprite))
  (Utilities|FlowControl|Sequence
    (:then_0
      (CallFunction|SetSpriteComponents))
    (:then_1
      (bind _children (CallFunction|GetChildrenSprites _rootsprite))
      (Variables|Default|SetOriginalSpriteComponents _children))
    (:then_2
      (CallFunction|CreateGrid (Variables|Default|GetAmountX) (Variables|Default|GetAmountZ) _rootsprite))))

(fn SetSpriteComponents
  (bind _hascutwall (Variables|Default|GetHasCutWall))
  (bind _piece2 (Variables|Default|GetPiece2))
  (bind _piece1 (Variables|Default|GetPiece1))
  (if (Variables|Default|GetHasGround)
    (if _hascutwall
      (Rendering|Components|Sprite|SetSprite _piece1 "/Game/Props/Sprites/Dungeon/_Ground_border_no_wall_Sprite._Ground_border_no_wall_Sprite")
      (Rendering|Components|Sprite|SetSprite _piece2 "/Game/Props/Sprites/Dungeon/_Cutwall2_Sprite._Cutwall2_Sprite" :!label _label)
      (else
        (Rendering|Components|Sprite|SetSprite _piece1 "/Game/Props/Sprites/Dungeon/_Ground_no_border_Sprite._Ground_no_border_Sprite")
        (Rendering|Components|Sprite|SetSprite _piece2 0 :!label _label_2)))
    (else
      (Rendering|Components|Sprite|SetSprite (Variables|Default|GetPiece1) 0)
      (if _hascutwall
        (goto _label)
        (else
          (goto _label_2)))))
  (return))

(fn CreateBlockCopy
  (params (IndexX :type Integer) (IndexZ :type Integer) (Root%20Sprite :type Paper%20Sprite%20Component%20Object%20Reference))
  (bind _copycenterrelativelocation (CallFunction|GetCopyCenter IndexX IndexZ Root%20Sprite))
  (Utilities|FlowControl|Sequence
    (:then_0
      ;[1 1 1] Copy center component
      (AddComponent|AddPaperSpriteComponent false _copycenterrelativelocation))
    (:then_1
      (CallFunction|CopySatelliteComponents _copycenterrelativelocation))))

(fn GetRepetitionScalars
  (Utilities|FlowControl|Sequence
    (:then_0
      (if (Variables|Default|GetRightwards)
        (LocalVariables|SetX 1)
        (else
          (LocalVariables|SetX -1))))
    (:then_1
      (if (Variables|Default|GetDownwards)
        (LocalVariables|SetZ -1)
        (else
          (LocalVariables|SetZ 1))))
    (:then_2
      (return (LocalVariables|GetX) (LocalVariables|GetZ)))))

(fn GetCloningDimensions
  (params (OriginalSprite :type Paper%20Sprite%20Component%20Object%20Reference))
  (bind _boxextent (Collision|GetComponentBounds OriginalSprite))
  (bind (_x _y _z) (Math|Vector|BreakVector _boxextent))
  (return (* 2 _x) (* 2 _z)))

(fn CreateGrid
  (params (AmountX :type Integer) (AmountZ :type Integer) (RootSprite :type Paper%20Sprite%20Component%20Object%20Reference))
  ;[1 1 1] Row creation loop
  (if (> AmountX 0)
    (for _index (range 0 (- AmountX 1))
      ;[1 1 1] Column creation loop
      (for _index_2 (range 0 AmountZ)
        (CallFunction|CreateBlockCopy _index _index_2 RootSprite)))
    (return)
    (else
      (for _index_3 (range 0 AmountZ)
        (CallFunction|CreateBlockCopy _index _index_3 RootSprite)))))

(fn GetCopyCenter
  (params (IndexX :type Integer) (IndexZ :type Integer) (OriginalSprite :type Paper%20Sprite%20Component%20Object%20Reference))
  (bind (_scalarx _scalarz) (CallFunction|GetRepetitionScalars))
  (bind (_dimensionx _dimensionz) (CallFunction|GetCloningDimensions OriginalSprite))
  (return (Math|Conversions|ToTransform(Vector) (Math|Vector|MakeVector (* (* IndexX _scalarx) _dimensionx) 0.0 (* (* IndexZ _scalarz) _dimensionz)))))

(fn GetChildrenSprites
  (params (RootSprite :type Scene%20Component%20Object%20Reference))
  (bind __children (LocalVariables|Get_Children))
  (for _array_element (Components|GetChildrenComponents RootSprite false)
    (bind _aspaper_sprite_component (Utilities|Casting|CastToPaperSpriteComponent _array_element)
      (:then
        (Utilities|Array|Add __children (Utilities|Struct|MakeSpriteComponent (Variables|/Script/Paper2D.PaperSpriteComponent|GetSourceSprite _aspaper_sprite_component) (Transformation|GetRelativeTransform _aspaper_sprite_component))))
      (:CastFailed
        (return __children))))
  (return __children))

(fn CopySatelliteComponents
  (params (InTransform :type Transform%20%28by%20ref%29))
  (for _array_element (Variables|Default|GetOriginalSpriteComponents)
    (bind _returnvalue (AddComponent|AddPaperSpriteComponent false (Math|Transform|MakeTransform (+ (.Location (Math|Transform|BreakTransform (.RelativeCoordinates (Utilities|Struct|BreakSpriteComponent _array_element)))) (.Location (Math|Transform|BreakTransform InTransform))) (.Rotation (Math|Transform|BreakTransform (.RelativeCoordinates (Utilities|Struct|BreakSpriteComponent _array_element)))) (.Scale (Math|Transform|BreakTransform (.RelativeCoordinates (Utilities|Struct|BreakSpriteComponent _array_element)))))))
    (Rendering|Components|Sprite|SetSprite _returnvalue (.Sprite (Utilities|Struct|BreakSpriteComponent _array_element))))
  (return))