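; Blade cutter trap built on a parent trap class, using 2D flipbooks, that kills the Prince and restarts the level.
; Flipbook-finished events chain closing, clang and reverse playback, repeating while prey is in range.
; Tick kills a Prince in KillingZone during the delayed lethal window, swaps to bloody flipbooks at the same frame, then reloads after death music.
; The construction script sets clean or bloodied blades, ground sprites and kill sound.
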(event OnComponentEndOverlap(KillingZone)
  (params (OtherActor :type Actor%20Object%20Reference) (OtherComp :type Primitive%20Component%20Object%20Reference) (OtherBodyIndex :type Integer))
  ;[1 1 1] Out the killing zone
  (Utilities|Casting|CastToPrinceCharacter OtherActor)
  (Variables|Default|SetPreyInKillingZone false))

(event OnComponentBeginOverlap(KillingZone)
  (params (OtherActor :type Actor%20Object%20Reference) (OtherComp :type Primitive%20Component%20Object%20Reference) (OtherBodyIndex :type Integer) (bFromSweep :type Boolean) (SweepResult :type Hit%20Result%20Structure%20%28by%20ref%29))
  ;[1 1 1] Into the killing zone
  (bind _asprince_character (Utilities|Casting|CastToPrinceCharacter OtherActor))
  (Utilities|FlowControl|Sequence
    (:then_0
      (Variables|Default|SetPreyInKillingZone true))
    (:then_1
      (Variables|Default|SetPrey _asprince_character))))

(event Custom|SpikesDeactivated
  ;[1 1 1] Blades deactivation
  (EventDispatchers|UnbindEventfromOnFinishedPlaying (Variables|Default|GetBackFlipbook) (delegate Custom|SpikesDeactivated))
  (if (Variables|Default|GetPreyInRange)
    (CallFunction|TrapActivated)
    (else
      (Variables|Default|SetCurrentState "NewEnumerator0"))))

(event Custom|SpikesFullyActivated
  ;[1 1 1] Blades activation
  (EventDispatchers|UnbindEventfromOnFinishedPlaying (Variables|Default|GetBackFlipbook) (delegate Custom|SpikesFullyActivated))
  (CallFunction|PlaySound (Variables|Default|GetBladesClangSound) (Variables|Default|GetAudio))
  (CallFunction|TrapDeactivated)
  (Variables|Default|SetCutterKilling false))

(event Custom|RestartLevel
  ;[1 1 1] Tick
  ;;[1 1 1] Restart level
  (EventDispatchers|UnbindEventfromOnAudioFinished (Variables|Default|GetAudio) (delegate Custom|RestartLevel))
  (CallFunction|ReloadLevel))

(event Custom|TrapDeactivated
  (bind _backflipbook (Variables|Default|GetBackFlipbook))
  ;[1 1 1] Blades deactivation
  (EventDispatchers|BindEventtoOnFinishedPlaying _backflipbook (delegate Custom|SpikesDeactivated))
  (Components|Timeline|ReversefromEnd _backflipbook)
  (Components|Timeline|ReversefromEnd (Variables|Default|GetFrontFlipbook)))

(event EventTrapActivated
  ;[1 1 1] Blades activation
  (EventDispatchers|BindEventtoOnFinishedPlaying (Variables|Default|GetBackFlipbook) (delegate Custom|SpikesFullyActivated))
  (Variables|Default|SetCurrentState "NewEnumerator2")
  (CallFunction|ActivateTrap false)
  (Utilities|FlowControl|Delay (Variables|Default|GetDelayBeforeKilling))
  (Variables|Default|SetCutterKilling true))

(event EventInitTrapActivation
  (params (PotentialVictim :type Actor%20Object%20Reference))
  ;[1 1 1] Entering blades range.
  (|CallParentFunction PotentialVictim)
  (Variables|Default|SetPreyInRange true))

(event EventInitTrapDeactivation
  (params (PotentialVictim :type Actor%20Object%20Reference))
  ;[1 1 1] Leaving blade range
  (|CallParentFunction PotentialVictim)
  (Variables|Default|SetPreyInRange false))

(event EventTick
  (params (DeltaSeconds :type Float%20%28single-precision%29))
  (bind _audio (Variables|Default|GetAudio))
  ;[1 1 1] Tick
  (if (Math|Boolean|ANDBoolean (Variables|Default|GetCutterKilling) (Variables|Default|GetPreyInKillingZone) (not (Variables|Default|GetAlreadyKilling)))
    (Variables|Default|SetAlreadyKilling true)
    (bind _asprince_character (Utilities|Casting|CastToPrinceCharacter (Variables|Default|GetPrey)))
    (Utilities|KillPrince _asprince_character self true
      (:Exit
        (Utilities|FlowControl|Sequence
          (:then_0
            (Variables|Default|SetPreyInKillingZone false)
            (CallFunction|BloodBlades)
            (Utilities|FlowControl|Delay 2.0)
            (Variables|Default|SetPreyInRange false)
            ;;[1 1 1] Restart level
            (CallFunction|PlaySound (Variables|Default|GetDeathMusic) _audio)
            (EventDispatchers|BindEventtoOnAudioFinished _audio (delegate Custom|RestartLevel))))))))

(fn ConstructionScript
  (Utilities|FlowControl|Sequence
    (:then_0
      ;[1 1 1] Blades visual setup.
      (if (Variables|Default|GetBloodSpoiled)
        (CallFunction|SetBladeFlipbooks (Variables|Default|GetBladesBloodSpoiledBack) (Variables|Default|GetBladesBloodSpoledFront))
        (else
          (CallFunction|SetBladeFlipbooks (Variables|Default|GetBladesCleanBack) (Variables|Default|GetBladesCleanFront))))
      (Audio|Components|Audio|Stop (Variables|Default|GetBackFlipbook))
      (Audio|Components|Audio|Stop (Variables|Default|GetFrontFlipbook)))
    (:then_1
      ;[1 1 1] Ground setup.
      (CallFunction|SetGroundSprites (Variables|Default|GetBladesGroundSprite) (Variables|Default|GetBladesGroundNoBorderSprite)))
    (:then_2
      ;[1 1 1] Audio setup.
      (Variables|Default|SetChaftSound (Variables|Default|GetBladesChaftSound)))
    (:then_3
      (|CallParentFunction))))

(fn SetBladeFlipbooks
  (params (BackFlipbook :type Paper%20Flipbook%20Object%20Reference) (FrontFlipbook :type Paper%20Flipbook%20Object%20Reference))
  (bind _output_get (Variables|Default|SetCurrentBackFlipbook BackFlipbook))
  (Sprite|SetFlipbook (Variables|Default|GetBackFlipbook) _output_get)
  (bind _output_get_2 (Variables|Default|SetCurrentFrontFlipbook FrontFlipbook))
  (Sprite|SetFlipbook (Variables|Default|GetFrontFlipbook) _output_get_2)
  (return))

(fn BloodBlades
  (bind _backflipbook (Variables|Default|GetBackFlipbook))
  (bind _frontflipbook (Variables|Default|GetFrontFlipbook))
  (if (and (!= (Variables|Default|GetCurrentFrontFlipbook) (Variables|Default|GetBladesBloodSpoledFront)) (!= (Variables|Default|GetCurrentBackFlipbook) (Variables|Default|GetBladesBloodSpoiledBack)))
    (LocalVariables|SetCurrentPlaybackPosition (Class|PaperFlipbookComponent|GetPlaybackPositioninFrames (Variables|Default|GetBackFlipbook)))
    ;[1 1 1] Flipbook components should be movable to allow change of flipbook at runtime.
    (CallFunction|SetBladeFlipbooks (Variables|Default|GetBladesBloodSpoiledBack) (Variables|Default|GetBladesBloodSpoledFront))
    (Utilities|FlowControl|Sequence
      (:then_0
        (Class|PaperFlipbookComponent|SetPlaybackPositioninFrames _backflipbook (LocalVariables|GetCurrentPlaybackPosition) false)
        (Audio|Components|Audio|Play _backflipbook))
      (:then_1
        (Class|PaperFlipbookComponent|SetPlaybackPositioninFrames _frontflipbook (LocalVariables|GetCurrentPlaybackPosition) false)
        (Audio|Components|Audio|Play _frontflipbook)))
    (else
      (Development|PrintString "Blood already set"))))